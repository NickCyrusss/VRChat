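; Floorplan measurement actor in the AVR navigation framework that maps between world and floorplan map space and registers itself with the main game state.
; Its construction script applies the floorplan texture to a plane through a dynamic material.
; Projection functions move a ReferenceScene component and read it back, though the transform variant returns a world transform.
; It also tests map objects against boxes tagged by map type and records map locations for its named floor.
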(event `self.ReceiveBeginPlay`
  (bind _game_state (`/Game/AVRFramework/Libraries/Lib_Core.getMainGameState` self))
  (`BlueprintSetLibrary.Set_Add` (`/Game/AVRFramework/Blueprints/Game/BP_GameState_Main.Floorplans` _game_state) self))

(fn `ComponentInsideMeasurement`
  (params (MapObject :type "Object Object Reference") (MapType :type "/Game/AVRFramework/Enums/Enum_Map_Type Enum" :default "NewEnumerator0"))
  (returns (IsInside :type Boolean))
  (bind _location (message `/Game/AVRFramework/Interface/Interface_MapInfo.Interface_GetMapLocation` MapObject))
  (for _array_element (`self.GetComponentsByTag` "/Script/Engine.BoxComponent" (`KismetStringLibrary.Conv_StringToName` (`|GetEnumeratorNameAsString` MapType)))
    (bind (_origin _boxextent) (`KismetSystemLibrary.GetComponentBounds` _array_element))
    (if (`KismetMathLibrary.IsPointInBox` _location _origin _boxextent)
      (return true)))
  (return false))

(fn `ProjectMapCoordinatesToWorld`
  (params (MapCoordinates :type "Vector Structure"))
  (returns (WorldCoordinates :type "Vector Structure"))
  (bind _referencescene (`self.ReferenceScene`))
  (bind (_returnvalue_x _returnvalue_y _returnvalue_z) (`KismetMathLibrary.BreakVector` (`SceneComponent.K2_GetComponentLocation` _referencescene)))
  (`SceneComponent.K2_SetRelativeLocation` _referencescene (`KismetMathLibrary.MakeVector` MapCoordinates_X MapCoordinates_Y MapCoordinates_Z) false false)
  (return (`KismetMathLibrary.MakeVector` _returnvalue_x _returnvalue_y _returnvalue_z)))

(fn `ProjectWorldCoordinatesToMap`
  (params (WorldCoordinates :type "Vector Structure"))
  (returns (MapCoordinates :type "Vector Structure"))
  (bind _referencescene (`self.ReferenceScene`))
  (bind (_relativelocation_x _relativelocation_y _relativelocation_z) (`KismetMathLibrary.BreakVector` (`SceneComponent.RelativeLocation` _referencescene)))
  (`SceneComponent.K2_SetWorldLocation` _referencescene (`KismetMathLibrary.MakeVector` WorldCoordinates_X WorldCoordinates_Y WorldCoordinates_Z) false false)
  (return (`KismetMathLibrary.MakeVector` _relativelocation_x _relativelocation_y _relativelocation_z)))

(fn `ProjectWorldRotationToMap`
  (params (WorldCoordinates :type "Rotator Structure"))
  (returns (MapCoordinates :type "Rotator Structure"))
  (bind _referencescene (`self.ReferenceScene`))
  (`SceneComponent.K2_SetWorldRotation` _referencescene WorldCoordinates false false)
  (return (`SceneComponent.RelativeRotation` _referencescene)))

(fn `ProjectWorldScaleToMap`
  (params (WorldCoordinates :type "Vector Structure"))
  (returns (MapCoordinates :type "Vector Structure"))
  (bind _referencescene (`self.ReferenceScene`))
  (`SceneComponent.SetWorldScale3D` _referencescene WorldCoordinates)
  (return (`SceneComponent.RelativeScale3D` _referencescene)))

(fn `ProjectWorldTransformToMap`
  (params (WorldCoordinates :type "Transform Structure"))
  (returns (MapCoordinates :type "Transform Structure"))
  (bind _referencescene (`self.ReferenceScene`))
  (`SceneComponent.K2_SetWorldTransform` _referencescene WorldCoordinates false false)
  (return (`SceneComponent.K2_GetComponentToWorld` _referencescene)))

(fn `SetComponentForFloor`
  (params (MapLocation :type "/Game/AVRFramework/Blueprints/Components/Util/Comp_MapLocation Object Reference") (Floor :type Name) (Set :type Boolean))
  (if (== Floor (`self.FloorName`))
    (`BlueprintMapLibrary.Map_Add` (`self.IsMapLocationOnFloor`) MapLocation Set)))

(fn `UserConstructionScript`
  (bind _returnvalue (`PrimitiveComponent.CreateDynamicMaterialInstance` (`self.Plane`) 0 null "None"))
  (`MaterialInstanceDynamic.SetTextureParameterValue` _returnvalue "MainTexture" (`self.Floorplan`))
  (`SceneComponent.SetVisibility` (`self.Plane`) (`self.Visible`) false))