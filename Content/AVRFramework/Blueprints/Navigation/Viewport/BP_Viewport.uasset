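; BP_Viewport is a placed navigation viewpoint in the AVR framework that supplies a captured preview of its view and teleports a pawn to its transform with a fade.
; GetView lazily claims the first unused index by scanning all viewport instances, captures the scene into that slot's render target from a fixed pool of twenty, and returns the Plane's dynamic material showing it.
; The teleport-surface query functions return only empty or false defaults.
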(event `self.ReceiveBeginPlay`)

(event `/Game/AVRFramework/Interface/Interface_Teleportable.TeleportTo`
  (params (Pawn :type "/Game/AVRFramework/Blueprints/Pawn/BP_Pawn_Base Object Reference") (ImpactLocation :type "Vector Structure") (UseRotation :type Boolean) (ImpactRotation :type "Rotator Structure"))
  ;[1 1 1] Teleport when Pressed
  (`/Game/AVRFramework/Blueprints/Pawn/BP_Pawn_Base.TeleportCharacter` Pawn (`self.K2_GetActorLocation`) (`self.K2_GetActorRotation`) 100.0 0.2 true false false true))

(fn `AssignFreeIndex`
  (locals (FreeIndexes :type "Array of Boolean"))
  (if (== (`self.Index`) -1)
    (bind _outactors (`GameplayStatics.GetAllActorsOfClass` "BP_Viewport_C"))
    (`KismetArrayLibrary.Array_Resize` (`local.FreeIndexes`) (`KismetArrayLibrary.Array_Length` _outactors))
    (for _array_element _outactors
      (bind _index (`/Game/AVRFramework/Blueprints/Navigation/Viewport/BP_Viewport.Index` _array_element))
      (if (not (== _index -1))
        (`KismetArrayLibrary.Array_Set` (`local.FreeIndexes`) _index true true)))
    (for (_array_element_2 _array_index) (`local.FreeIndexes`)
      (if (not _array_element_2)
        (set `self.Index` _array_index)
        (return))))
  (return))

(fn `AssignRenderTarget`
  (params (Index :type Integer)))

(fn `CanTeleport`
  (returns (CanTeleport :type Boolean))
  (return false))

(fn `getClosestTeleportImpactPoint`
  (params (ReferenceLocation :type "Vector Structure"))
  (returns (ClosestLocation :type "Vector Structure"))
  (return (0.0 0.0 0.0)))

(fn `getTeleportFloor`
  (returns (Floorname :type Name) (Universal :type Boolean))
  (return "None" false))

(fn `getView`
  (returns (Material :type "MaterialInterface Object Reference"))
  (bind _scenecapture (`self.SceneCapture`))
  (bind _plane (`self.Plane`))
  (bind _returnvalue (select `int` (`self.Index`) :`0` "/Game/AVRFramework/Materials/Viewports/RT_Framework_Viewport_00.RT_Framework_Viewport_00" :`1` "/Game/AVRFramework/Materials/Viewports/RT_Framework_Viewport_01.RT_Framework_Viewport_01" :`2` "/Game/AVRFramework/Materials/Viewports/RT_Framework_Viewport_02.RT_Framework_Viewport_02" :`3` "/Game/AVRFramework/Materials/Viewports/RT_Framework_Viewport_03.RT_Framework_Viewport_03" :`4` "/Game/AVRFramework/Materials/Viewports/RT_Framework_Viewport_04.RT_Framework_Viewport_04" :`5` "/Game/AVRFramework/Materials/Viewports/RT_Framework_Viewport_05.RT_Framework_Viewport_05" :`6` "/Game/AVRFramework/Materials/Viewports/RT_Framework_Viewport_06.RT_Framework_Viewport_06" :`7` "/Game/AVRFramework/Materials/Viewports/RT_Framework_Viewport_07.RT_Framework_Viewport_07" :`8` "/Game/AVRFramework/Materials/Viewports/RT_Framework_Viewport_08.RT_Framework_Viewport_08" :`9` "/Game/AVRFramework/Materials/Viewports/RT_Framework_Viewport_09.RT_Framework_Viewport_09" :`10` "/Game/AVRFramework/Materials/Viewports/RT_Framework_Viewport_10.RT_Framework_Viewport_10" :`11` "/Game/AVRFramework/Materials/Viewports/RT_Framework_Viewport_11.RT_Framework_Viewport_11" :`12` "/Game/AVRFramework/Materials/Viewports/RT_Framework_Viewport_12.RT_Framework_Viewport_12" :`13` "/Game/AVRFramework/Materials/Viewports/RT_Framework_Viewport_13.RT_Framework_Viewport_13" :`14` "/Game/AVRFramework/Materials/Viewports/RT_Framework_Viewport_14.RT_Framework_Viewport_14" :`15` "/Game/AVRFramework/Materials/Viewports/RT_Framework_Viewport_15.RT_Framework_Viewport_15" :`16` "/Game/AVRFramework/Materials/Viewports/RT_Framework_Viewport_16.RT_Framework_Viewport_16" :`17` "/Game/AVRFramework/Materials/Viewports/RT_Framework_Viewport_17.RT_Framework_Viewport_17" :`18` "/Game/AVRFramework/Materials/Viewports/RT_Framework_Viewport_18.RT_Framework_Viewport_18" :`19` "/Game/AVRFramework/Materials/Viewports/RT_Framework_Viewport_19.RT_Framework_Viewport_19" :!type "TextureRenderTarget2D Object Reference"))
  ;[1 1 1] get View from the Current Viewport
  (`self.AssignFreeIndex`)
  (set `SceneCaptureComponent2D.TextureTarget` _returnvalue _scenecapture)
  (`SceneCaptureComponent2D.CaptureScene` _scenecapture)
  (bind _returnvalue_2 (`PrimitiveComponent.CreateDynamicMaterialInstance` _plane 0 null "None"))
  (`MaterialInstanceDynamic.SetTextureParameterValue` _returnvalue_2 "Texture" _returnvalue)
  (return (`PrimitiveComponent.GetMaterial` _plane 0)))

(fn `UserConstructionScript`)