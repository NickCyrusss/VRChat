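; BP_SpectatorPosition is a placeable marker for an indexed spectator position in the AVRFramework navigation system.
; Its Construction Script shows the Index on a TextRender component as a label.
; It then scans all other BP_SpectatorPosition actors and prints a warning if one already uses the same Index, without changing the value.
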(fn `UserConstructionScript`
  (`TextRenderComponent.K2_SetText` (`self.TextRender`) (`KismetTextLibrary.Conv_IntToText` (`self.Index`)))
  ;[1 1 1] Index security Check
  (bind _outactors (`GameplayStatics.GetAllActorsOfClass` "BP_SpectatorPosition_C"))
  (for _array_element _outactors
    (if (!= _array_element self)
      (if (== (`/Game/AVRFramework/Blueprints/Navigation/BP_SpectatorPosition.Index` _array_element) (`self.Index`))
        (`KismetSystemLibrary.PrintString` "This spectator Index is already taken")))))