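; Actor component in the AVRFramework that provides an IsOwner check for whether the local machine controls the actor it is attached to.
; IsOwner inspects that actor's owner, returning local-controller status for a PlayerController or locally-controlled status for a Pawn.
; With no valid owner, or one of another type, it falls back to whether the actor has authority.
; The event graph holds no active logic.
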(fn `isOwner`
  (returns (Owner :type Boolean))
  (bind _returnvalue (`self.GetOwner`))
  (bind _returnvalue_2 (`Actor.GetOwner` _returnvalue))
  (`/Engine/EditorBlueprintResources/StandardMacros.IsValid` _returnvalue_2
    (:`Is Valid`
      (bind _asplayer_controller (cast `PlayerController` _returnvalue_2)
        (:`then`
          (return (`Controller.IsLocalPlayerController` _asplayer_controller)))
        (:`CastFailed`
          (bind _aspawn (cast `Pawn` _returnvalue_2)
            (:`then`
              (return (`Pawn.IsLocallyControlled` _aspawn)))
            (:`CastFailed`
              _)))))
    (:`Is Not Valid`
      _))
  (return (`Actor.HasAuthority` _returnvalue)))