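; BP_ExtendablePointer is a grabbable VR pointer device that telescopes in and out when toggled.
; A Trigger key from the grab component toggles the active component.
; Active state changes play or reverse a timeline that drives a morph target on the pointer mesh.
; The construction-time active state event also jumps the timeline to the matching end state.
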(event `self.Comp_Active.ConstActiveStateChanged`
  (params (Active :type Boolean))
  (`/Game/AVRFramework/Libraries/MLib_Object_Macros.ManipulateTimeline` (`self.ExtendPointer`) Active)
  ;[1 1 1] Expand on Trigger
  (`SkeletalMeshComponent.SetMorphTarget` (`self.ExtendablePointer`) "pCylinder8" (stale `self.Comp_Active.ActiveStateChanged` _extend) true :!label _label))

(event `self.Comp_Active.ActiveStateChanged`
  (params (Active :type Boolean))
  ;[1 1 1] Expand on Trigger
  (if Active
    (bind (_direction _extend) (`Timeline|ExtendPointer` :!label _label_2)
      (:`Update`
        (goto _label)))
    (else
      (goto _label_2 :!via `Reverse`))))

(event `self.Comp_Grab.KeyInput`
  (params (Key :type "/Game/AVRFramework/Enums/Enum_Controller_Buttons Enum" :default "NewEnumerator1") (Set :type Boolean))
  ;[1 1 1] Key Input
  (switch `/Game/AVRFramework/Enums/Enum_Controller_Buttons` Key
    (:`NewEnumerator0`
      (`/Game/AVRFramework/Blueprints/Components/State/Comp_Active.ToggleActiv` (`self.Comp_Active`)))))

(fn `UserConstructionScript`)