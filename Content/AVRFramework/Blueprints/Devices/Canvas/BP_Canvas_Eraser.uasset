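; Grabbable VR eraser that wipes a canvas by painting white strokes where its box crosses the canvas plane.
; Box overlap caches the Comp_Child_Canvas, so Tick only works during contact.
; Each tick, an Arrow steps across a density-based grid over the box, and its line-plane intersections become short, randomly jittered strokes through the canvas's Paint.
; The grabbing motion controller gets haptic feedback while erasing.
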(event `self.Box.OnComponentBeginOverlap`
  (params (OverlappedComponent :type "PrimitiveComponent Object Reference") (OtherActor :type "Actor Object Reference") (OtherComp :type "PrimitiveComponent Object Reference") (OtherBodyIndex :type Integer) (bFromSweep :type Boolean) (SweepResult :type "HitResult Structure (by ref)"))
  ;[1 1 1] Only Trace when actually overlapping with Canvas
  (bind _ascomp_child_canvas (cast `/Game/AVRFramework/Blueprints/Components/ChildActor/Comp_Child_Canvas` OtherActor))
  (set `self.Canvas` _ascomp_child_canvas))

(event `self.Box.OnComponentEndOverlap`
  (params (OverlappedComponent :type "PrimitiveComponent Object Reference") (OtherActor :type "Actor Object Reference") (OtherComp :type "PrimitiveComponent Object Reference") (OtherBodyIndex :type Integer))
  ;[1 1 1] Only Trace when actually overlapping with Canvas
  (if (== OtherActor (`self.Canvas`))
    (set `self.Canvas` null)))

(event `self.ReceiveTick`
  (params (DeltaSeconds :type "Float (single-precision)"))
  (bind _arrow (`self.Arrow`))
  (bind _returnvalue (/ 1.0 (`self.DensityPerCM`)))
  (bind _returnvalue_2 (`SceneComponent.K2_GetComponentLocation` _arrow))
  (bind _canvas (`/Game/AVRFramework/Blueprints/Components/ChildActor/Comp_Child_Canvas.Canvas` (`self.Canvas`)))
  (bind (_boxextent_x _boxextent_y _boxextent_z) (`KismetMathLibrary.BreakVector` (`BoxComponent.BoxExtent` (`self.Box`))))
  (bind _canvas_2 (`/Game/AVRFramework/Blueprints/Components/ChildActor/Comp_Child_Canvas.Canvas` (`self.Canvas`)))
  (bind _returnvalue_3 (* _returnvalue -1.0))
  (bind _returnvalue_4 (`KismetMathLibrary.FTrunc` (* _boxextent_y (`self.DensityPerCM`))))
  (bind _returnvalue_5 (`KismetMathLibrary.FTrunc` (* _boxextent_x (`self.DensityPerCM`))))
  (bind (_t _intersection _returnvalue_6) (`KismetMathLibrary.LinePlaneIntersection` _returnvalue_2 (+ _returnvalue_2 (* (`SceneComponent.GetForwardVector` _arrow) (* _boxextent_z 2.0))) (`KismetMathLibrary.MakePlaneFromPointAndNormal` (`SceneComponent.K2_GetComponentLocation` _canvas_2) (`SceneComponent.GetForwardVector` _canvas_2))))
  ;[1 1 1] Calculate intersecting locations to erase
  (`/Engine/EditorBlueprintResources/StandardMacros.IsValid` (`self.Canvas`)
    (:`Is Valid`
      (for _index (range (+ _returnvalue_5 1))
        (for _index_2 (range (+ _returnvalue_4 1))
          (`SceneComponent.K2_SetRelativeLocation` (`self.Arrow`) (`KismetMathLibrary.MakeVector` (`self.ValueRelativeToIndex` _index _returnvalue_5 _boxextent_x) (`self.ValueRelativeToIndex` _index_2 _returnvalue_4 _boxextent_y) _boxextent_z) false false)
          (if _returnvalue_6
            (`/Game/AVRFramework/Blueprints/Components/ChildActor/Comp_Child_Canvas.Paint` (`self.Canvas`) _intersection (+ _intersection (+ (* (`SceneComponent.GetUpVector` _canvas) (`KismetMathLibrary.RandomFloatInRange` _returnvalue_3 _returnvalue)) (* (`SceneComponent.GetRightVector` _canvas) (`KismetMathLibrary.RandomFloatInRange` _returnvalue_3 _returnvalue)))) 5.0 (struct :`R` 1.0 :`G` 1.0 :`B` 1.0 :`A` 1.0)))))
      (`/Game/AVRFramework/Libraries/Lib_Core.SetHaptics` (`/Game/AVRFramework/Blueprints/Components/Interaction/Comp_Grab.GrabbingMotionController` (`self.Comp_Grab`)) "NewEnumerator1" "NewEnumerator4" 0.0 0.4))))

(fn `getRelativeLaserPosition`
  (returns (RelativeLocation :type "Transform Structure"))
  (return (`KismetMathLibrary.MakeTransform` (2.0 0.0 0.0) (struct :`Pitch` 90.0))))

(fn `UserConstructionScript`)