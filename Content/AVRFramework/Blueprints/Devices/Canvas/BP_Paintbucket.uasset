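; BP_Paintbucket is a paint bucket that gives an overlapping BP_Canvas_Marker its color.
; The construction script tints the bucket through a dynamic material instance.
; On sphere overlap it recolors the marker and plays a tinted splash particle and sound, with a DoOnce and short delay as a retrigger cooldown.
; While a marker is inside, Tick writes its tip position to MPC_Paintbucket, which is cleared on exit.
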(event `self.ReceiveTick`
  (params (DeltaSeconds :type "Float (single-precision)"))
  ;[1 1 1] Modify Paint if Brush is close
  (bind _marker (`self.Marker`)
    (:`then`
      (`KismetMaterialLibrary.SetVectorParameterValue` "/Game/AVRFramework/Meshes/Devices/Paintbucket/MPC_Paintbucket.MPC_Paintbucket" "penlocation" (`KismetMathLibrary.Conv_VectorToLinearColor` (`SceneComponent.K2_GetComponentLocation` (`/Game/AVRFramework/Blueprints/Devices/Canvas/BP_Canvas_Marker.Tip` _marker)))))
    (:`else`)))

(event `self.Sphere.OnComponentBeginOverlap`
  (params (OverlappedComponent :type "PrimitiveComponent Object Reference") (OtherActor :type "Actor Object Reference") (OtherComp :type "PrimitiveComponent Object Reference") (OtherBodyIndex :type Integer) (bFromSweep :type Boolean) (SweepResult :type "HitResult Structure (by ref)"))
  (bind _color (`self.Color`))
  (bind _returnvalue (`SceneComponent.K2_GetComponentLocation` (`self.ParticleLocation`)))
  ;[1 1 1] Start Overlap
  (bind _asbp_canvas_marker (cast `/Game/AVRFramework/Blueprints/Devices/Canvas/BP_Canvas_Marker` OtherActor))
  (set `self.Marker` _asbp_canvas_marker)
  (`/Engine/EditorBlueprintResources/StandardMacros.DoOnce` false :!label _label
    (:`Completed`
      (set `/Game/AVRFramework/Blueprints/Devices/Canvas/BP_Canvas_Marker.Color` _color _asbp_canvas_marker)
      (`/Game/AVRFramework/Blueprints/Devices/Canvas/BP_Canvas_Marker.UpdateColor` _asbp_canvas_marker)
      (bind _returnvalue_2 (`GameplayStatics.SpawnEmitterAtLocation` "/Game/AVRFramework/Meshes/Devices/Paintbucket/P_Paintbucket_Splashed.P_Paintbucket_Splashed" _returnvalue))
      (`ParticleSystemComponent.SetColorParameter` _returnvalue_2 "color" _color)
      (`GameplayStatics.PlaySoundAtLocation` "/Game/AVRFramework/Sound/Waves/Tools/Paintbucket/SplashSound.SplashSound" _returnvalue (struct) 1.0 1.0 0.0 "/Game/AVRFramework/Sound/Attenuation/Atten_UI_3D.Atten_UI_3D" null null)
      (`KismetSystemLibrary.Delay` 0.2)
      (`self.OnRetrigger`))))

(event `OnRetrigger`
  ;[1 1 1] Start Overlap
  (goto _label :!via `Reset`))

(event `self.Sphere.OnComponentEndOverlap`
  (params (OverlappedComponent :type "PrimitiveComponent Object Reference") (OtherActor :type "Actor Object Reference") (OtherComp :type "PrimitiveComponent Object Reference") (OtherBodyIndex :type Integer))
  ;[1 1 1] Invalidate Marker
  (if (== OtherActor (`self.Marker`))
    (set `self.Marker` null)
    (`KismetMaterialLibrary.SetVectorParameterValue` "/Game/AVRFramework/Meshes/Devices/Paintbucket/MPC_Paintbucket.MPC_Paintbucket" "penlocation" (make `LinearColor` 0.0))))

(fn `UserConstructionScript`
  (bind _returnvalue (`PrimitiveComponent.CreateDynamicMaterialInstance` (`self.Paintbucket`) 0 null "None"))
  (`MaterialInstanceDynamic.SetVectorParameterValue` _returnvalue "Color" (`self.Color`)))