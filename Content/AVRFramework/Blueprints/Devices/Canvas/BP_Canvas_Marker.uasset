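; VR marker that paints on canvas actors, with an optional detachable cap and adjustable color.
; The authority spawns the cap on an anchor; attaching or detaching it toggles its physics.
; When an uncapped tip capsule begins overlapping a canvas, Tick sphere-traces the capsule, paints lines between successive hit points and pulses controller haptics.
; Thumbstick input adjusts thickness and tip scale, while UpdateColor recolors marker, tip and attached cap.
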(event `self.ReceiveBeginPlay`
  (bind _reprcap (`self.ReprCap`))
  ;[1 1 1] Begin Play Cap
  (`/Engine/EditorBlueprintResources/ActorMacros.Switch Has Authority`
    (:`Authority`
      (`|ExecutionSequence`
        (:`then_0`
          (if (`self.HasCap`)
            (bind _returnvalue (`|SpawnActorFromClass` "/Game/AVRFramework/Blueprints/Devices/Canvas/BP_Canvas_Marker_Cap.BP_Canvas_Marker_Cap_C" (`SceneComponent.K2_GetComponentToWorld` (`self.ReprCap`)) "AlwaysSpawn" "OverrideRootScale" null (`self.Color`) null))
            (bind _output_get (set `self.Cap` _returnvalue))
            (`/Game/AVRFramework/Blueprints/Components/Snapping/Comp_Connector.AttachConnectorToActor` (`/Game/AVRFramework/Blueprints/Devices/Canvas/BP_Canvas_Marker_Cap.BP_Comp_Connector_Anchor` _output_get) self (`self.Comp_Anchor`) "None" (`SceneComponent.K2_GetComponentToWorld` (`self.ReprCap`)))
            (`/Game/AVRFramework/Blueprints/Components/Util/Comp_Anchor.OccupyAnchor` (`self.Comp_Anchor`) _output_get)))
        (:`then_1`
          (`/Engine/EditorBlueprintResources/StandardMacros.IsValid` _reprcap :!label _label
            (:`Is Valid`
              (`ActorComponent.K2_DestroyComponent` _reprcap))))))
    (:`Remote`
      (goto _label))))

(event `self.Comp_Attach.ActorAttached`
  (params (NewlyAttachedActor :type "Actor Object Reference"))
  (bind _asbp_canvas_marker_cap (cast `/Game/AVRFramework/Blueprints/Devices/Canvas/BP_Canvas_Marker_Cap` NewlyAttachedActor))
  (bind _output_get (set `self.Cap` _asbp_canvas_marker_cap))
  (bind _cap (`/Game/AVRFramework/Blueprints/Devices/Canvas/BP_Canvas_Marker_Cap.Cap` _output_get))
  (`PrimitiveComponent.SetCollisionEnabled` _cap "QueryOnly")
  (`PrimitiveComponent.SetSimulatePhysics` _cap false))

(event `self.Comp_Attach.ActorDetached`
  (params (DetachedActor :type "Actor Object Reference"))
  (bind _asbp_canvas_marker_cap (cast `/Game/AVRFramework/Blueprints/Devices/Canvas/BP_Canvas_Marker_Cap` DetachedActor))
  (set `self.Cap` null)
  (bind _cap (`/Game/AVRFramework/Blueprints/Devices/Canvas/BP_Canvas_Marker_Cap.Cap` _asbp_canvas_marker_cap))
  (`PrimitiveComponent.SetCollisionEnabled` _cap "QueryAndPhysics")
  (`PrimitiveComponent.SetSimulatePhysics` _cap true))

(event `self.ReceiveTick`
  (params (DeltaSeconds :type "Float (single-precision)"))
  (bind _capsule (`self.Capsule`))
  (bind _returnvalue (`SceneComponent.K2_GetComponentLocation` (`self.Capsule`)))
  (bind _returnvalue_2 (* (`SceneComponent.GetUpVector` _capsule) (`CapsuleComponent.CapsuleHalfHeight` _capsule)))
  ;[1 1 1] Trace and Draw when overlapping with Canvas
  (`/Engine/EditorBlueprintResources/StandardMacros.IsValid` (`self.Canvas`)
    (:`Is Valid`
      (bind _outhits (`KismetSystemLibrary.SphereTraceMulti` (- _returnvalue _returnvalue_2) (+ _returnvalue _returnvalue_2) (`CapsuleComponent.CapsuleRadius` _capsule) "TraceTypeQuery1" false (`|MakeArray` self :!type "Actor Object Reference")))
      (for _array_element _outhits
        (bind (_bblockinghit _binitialoverlap _time _distance _location _impactpoint _normal _impactnormal _physmat _hitactor) (`GameplayStatics.BreakHitResult` _array_element))
        (bind _ascomp_child_canvas (cast `/Game/AVRFramework/Blueprints/Components/ChildActor/Comp_Child_Canvas` _hitactor))
        (`/Game/AVRFramework/Blueprints/Components/ChildActor/Comp_Child_Canvas.Paint` _ascomp_child_canvas (`self.PreviousDrawLocation`) _impactpoint (`self.Thickness`) (`self.Color`))
        (set `self.PreviousDrawLocation` _impactpoint))
      (`/Game/AVRFramework/Libraries/Lib_Core.SetHaptics` (`/Game/AVRFramework/Blueprints/Components/Interaction/Comp_Grab.GrabbingMotionController` (`self.Comp_Grab`)) "NewEnumerator1" "NewEnumerator4" 0.0 0.15))))

(event `self.Capsule.OnComponentBeginOverlap`
  (params (OverlappedComponent :type "PrimitiveComponent Object Reference") (OtherActor :type "Actor Object Reference") (OtherComp :type "PrimitiveComponent Object Reference") (OtherBodyIndex :type Integer) (bFromSweep :type Boolean) (SweepResult :type "HitResult Structure (by ref)"))
  ;[1 1 1] Only Draw when overlapping with Canvas
  (`/Engine/EditorBlueprintResources/StandardMacros.IsValid` (`self.Cap`)
    (:`Is Not Valid`
      (bind _ascomp_child_canvas (cast `/Game/AVRFramework/Blueprints/Components/ChildActor/Comp_Child_Canvas` OtherActor))
      (set `self.Canvas` _ascomp_child_canvas)
      (set `self.PreviousDrawLocation` (`SceneComponent.K2_GetComponentLocation` (`self.Capsule`))))))

(event `self.Capsule.OnComponentEndOverlap`
  (params (OverlappedComponent :type "PrimitiveComponent Object Reference") (OtherActor :type "Actor Object Reference") (OtherComp :type "PrimitiveComponent Object Reference") (OtherBodyIndex :type Integer))
  ;[1 1 1] Only Draw when overlapping with Canvas
  (if (== OtherActor (`self.Canvas`))
    (set `self.Canvas` null)))

(event `self.Comp_Grab.Thumbstick`
  (params (UpAxis :type "Float (single-precision)") (RightAxis :type "Float (single-precision)"))
  (bind _relativescale3d_x (`KismetMathLibrary.BreakVector` (`SceneComponent.RelativeScale3D` (`self.Tip`))))
  ;[1 1 1] Set Thickness of the Marker
  (bind _output_get (set `self.Thickness` (`KismetMathLibrary.FClamp` (+ (`self.Thickness`) RightAxis) 2.0 20.0)))
  (bind _returnvalue (`KismetMathLibrary.MapRangeClamped` _output_get 2.0 20.0 0.3 1.4))
  (`SceneComponent.SetRelativeScale3D` (`self.Tip`) (`KismetMathLibrary.MakeVector` _relativescale3d_x _returnvalue _returnvalue)))

(event `UpdateColor`
  (bind _cap (`self.Cap`))
  (bind _returnvalue (`KismetMathLibrary.Conv_LinearColorToVector` (`self.Color`)))
  ;[1 1 1] Update Color (Bucket)
  (`/Engine/EditorBlueprintResources/StandardMacros.IsValid` _cap
    (:`Is Valid`
      (`MeshComponent.SetVectorParameterValueOnMaterials` (`/Game/AVRFramework/Blueprints/Devices/Canvas/BP_Canvas_Marker_Cap.Cap` _cap) "Color" _returnvalue))
    (:`Is Not Valid`
      _))
  (`MeshComponent.SetVectorParameterValueOnMaterials` (`self.Marker`) "Color" _returnvalue)
  (`MeshComponent.SetVectorParameterValueOnMaterials` (`self.Tip`) "Color" (/ _returnvalue 3.0)))

(fn `getRelativeLaserPosition`
  (returns (RelativeLocation :type "Transform Structure"))
  (return (`KismetMathLibrary.MakeTransform` (0.0 0.0 0.0) (struct :`Roll` 90.0))))

(fn `UserConstructionScript`
  (bind _reprcap (`self.ReprCap`))
  (bind _returnvalue (`KismetMathLibrary.Conv_LinearColorToVector` (`self.Color`)))
  (`MeshComponent.SetVectorParameterValueOnMaterials` (`self.ReprCap`) "Color" _returnvalue)
  (`MeshComponent.SetVectorParameterValueOnMaterials` (`self.Marker`) "Color" _returnvalue)
  (`MeshComponent.SetVectorParameterValueOnMaterials` (`self.Tip`) "Color" (/ _returnvalue 3.0))
  (if (not (`self.HasCap`))
    (`/Engine/EditorBlueprintResources/StandardMacros.IsValid` _reprcap
      (:`Is Valid`
        (`ActorComponent.K2_DestroyComponent` _reprcap)))))