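; BP_Device_Camera is a grabbable VR camera that takes photos, with selfie and gallery modes.
; While held and outside gallery mode, it captures a low-res preview every tick, and the trigger spawns a BP_Helper_Photo whose render target receives a high-res capture, with shutter sound and haptics.
; Face buttons toggle selfie mode, which flips the capture handle, and gallery mode, which shows a widget and swaps the screen material.
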(event `self.ReceiveBeginPlay`
  ;[1 1 1] Initialize
  (`parent.ReceiveBeginPlay`)
  (`self.SetGalleryMode` (`self.GalleryMode`)))

(event `self.ReceiveTick`
  (params (DeltaSeconds :type "Float (single-precision)"))
  (`parent.ReceiveTick` DeltaSeconds)
  ;[1 1 1] When active Capture Scene and Update Display
  (if (`/Game/AVRFramework/Blueprints/Components/State/Comp_Active.Active` (`self.Comp_Active`))
    (if (not (`self.GalleryMode`))
      (set `TextureRenderTarget.TargetGamma` 2.0 (`SceneCaptureComponent2D.TextureTarget` (`self.SceneCaptureComponent2DLowres`)))
      (`SceneCaptureComponent2D.CaptureScene` (`self.SceneCaptureComponent2DLowres`)))))

(event `self.Comp_Grab.ActorPickedUp`
  (params (GrabbingPawn :type "/Game/AVRFramework/Blueprints/Pawn/BP_Pawn_Base Object Reference") (GrabbingActor :type "Actor Object Reference") (GrabbingMotionController :type "/Game/AVRFramework/Blueprints/VR/MotionControllers/BP_MotionController Object Reference") (GrabbingMComp :type "/Game/AVRFramework/Blueprints/VR/MotionComponents/BP_MComp Object Reference"))
  ;[1 1 1] Handle Grab - Activates on Grab
  (`/Game/AVRFramework/Blueprints/Components/State/Comp_Active.SetActiv` (`self.Comp_Active`) true))

(event `SetGalleryMode`
  (params (GalleryMode :type Boolean))
  ;[1 1 1] GalleryMode
  (bind _output_get (set `self.GalleryMode` GalleryMode))
  (`SceneComponent.SetVisibility` (`self.Comp_Widget`) _output_get false)
  (`PrimitiveComponent.SetMaterial` (`self.Camera`) 5 (select `bool` _output_get :`false` "/Game/AVRFramework/Blueprints/Devices/Camera/Mat_Camera.Mat_Camera" :`true` "/Game/AVRFramework/Meshes/Devices/Tablet/Mat_Device_Tablet_Plastic_Black.Mat_Device_Tablet_Plastic_Black" :!type "MaterialInterface Object Reference")))

(event `self.Comp_Grab.ActorReleased`
  (params (ReleasingPawn :type "/Game/AVRFramework/Blueprints/Pawn/BP_Pawn_Base Object Reference") (ReleasingActor :type "Actor Object Reference") (ReleasingMotionController :type "/Game/AVRFramework/Blueprints/VR/MotionControllers/BP_MotionController Object Reference") (ReleasingMComp :type "/Game/AVRFramework/Blueprints/VR/MotionComponents/BP_MComp Object Reference"))
  ;[1 1 1] Handle Grab - Activates on Grab
  (`/Game/AVRFramework/Blueprints/Components/State/Comp_Active.SetActiv` (`self.Comp_Active`) false))

(event `self.Comp_Grab.KeyInput`
  (params (Key :type "/Game/AVRFramework/Enums/Enum_Controller_Buttons Enum" :default "NewEnumerator1") (Set :type Boolean))
  ;[1 1 1] Take Photo on Trigger Pressed, taking Pictures creates a Photo Actor
  (switch `/Game/AVRFramework/Enums/Enum_Controller_Buttons` Key
    (:`NewEnumerator0`
      (if Set
        (if (not (`self.GalleryMode`))
          (`self.TakePicture`))))
    (:`NewEnumerator3`
      (if Set
        (`self.SetSelfieMode` (not (`self.SelfieMode`)))))
    (:`NewEnumerator4`
      (if Set
        (`self.SetGalleryMode` (not (`self.GalleryMode`)))))))

(event `SetSelfieMode`
  (params (Set :type Boolean))
  ;[1 1 1] Take Photo on Trigger Pressed, taking Pictures creates a Photo Actor
  (set `self.SelfieMode` Set)
  (`KismetSystemLibrary.MoveComponentTo` (`self.CaptureHandle`) (select `bool` Set :`false` (0.0 0.0 -3.0) :`true` (0.0 0.0 3.0) :!type "Vector Structure") (select `bool` Set :`false` (struct :`Pitch` -90.0 :`Roll` 180.0) :`true` (struct :`Pitch` 90.0) :!type "Rotator Structure") true true 0.3 true))

(event `TakePicture`
  (bind _scenecapturecomponent2dhighres (`self.SceneCaptureComponent2DHighres`))
  ;[1 1 1] Take Photo on Trigger Pressed, taking Pictures creates a Photo Actor
  (bind _returnvalue (`|SpawnActorFromClass` "/Game/AVRFramework/Blueprints/Helpers/BP_Helper_Photo.BP_Helper_Photo_C" (`KismetMathLibrary.MakeTransform` (0.0 0.0 10000.0)) "AlwaysSpawn" "OverrideRootScale" null "Photo" "This is a Photo" null))
  (bind _texturetarget (`/Game/AVRFramework/Blueprints/Helpers/BP_Helper_Photo.PrintPicture` _returnvalue))
  (set `TextureRenderTarget.TargetGamma` 2.5 _texturetarget)
  (set `SceneCaptureComponent2D.TextureTarget` _texturetarget _scenecapturecomponent2dhighres)
  (`SceneCaptureComponent2D.CaptureScene` _scenecapturecomponent2dhighres)
  (`GameplayStatics.PlaySoundAtLocation` "/Game/AVRFramework/Sound/Cues/Device/Camera/Cue_Device_Camera.Cue_Device_Camera" (`self.K2_GetActorLocation`) (struct) 1.0 1.0 0.0 null null null)
  (`self.PictureTaken`)
  (`/Game/AVRFramework/Libraries/Lib_Core.SetHaptics` (`/Game/AVRFramework/Blueprints/Components/Interaction/Comp_Grab.GrabbingMotionController` (`self.Comp_Grab`)) "NewEnumerator1" "NewEnumerator2" 0.1 1.0))

(fn `UserConstructionScript`
  (`parent.UserConstructionScript`))