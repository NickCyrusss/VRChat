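; VR player pawn that spawns swappable left and right motion controller actors and forwards buttons, axes, and thumbstick directions (also as button presses) to them.
; It sets tracking origin per HMD, fits capsule height to the camera, and recenters the capsule before teleports.
; Keyboard and mouse drive camera or hands under manual control, or a spawned spectator pawn.
; In-development spectator modes switch screen layouts and jump between placed positions.
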(event `InputAction|MotionControllerTriggerLeft`
  (params (Key :type "Key Structure"))
  ;[1 1 1] Forward Inputs to Motion Controller
  (:`Pressed`
    (`self.SetButtonSet` "NewEnumerator0" :!label _label))
  (:`Released`
    (goto _label :!via `LeftReleased`)))

(event `InputAxis|CapTouchPointingLeft`
  (params (AxisValue :type "Float (single-precision)"))
  ;[1 1 1] Forward Inputs to Motion Controller
  (bind _controller (`self.GetController` "NewEnumerator0")
    (:`found`
      (`/Game/AVRFramework/Blueprints/VR/MotionControllers/BP_MotionController.TriggerCapTouch` _controller AxisValue))))

(event `InputAction|FaceButton01Left`
  (params (Key :type "Key Structure"))
  ;[1 1 1] Forward Inputs to Motion Controller
  (:`Pressed`
    (`self.SetButtonSet` "NewEnumerator3" :!label _label_2))
  (:`Released`
    (goto _label_2 :!via `LeftReleased`)))

(event `InputAxis|LookUp`
  (params (AxisValue :type "Float (single-precision)"))
  (bind _returnvalue (`self.CurrentlyFocusedComponent`))
  (bind (_relativerotation_roll _relativerotation_pitch) (`KismetMathLibrary.BreakRotator` (`SceneComponent.RelativeRotation` _returnvalue)))
  ;[1 1 1] Keyboard Inputs For Spectator
  (bind _spectator (`self.Spectator`)
    (:`then`
      (`/Game/AVRFramework/Blueprints/Pawn/BP_Pawn_NonVR.LookUp` _spectator AxisValue))
    (:`else`
      (`self.HasManualControl`
        (:`true`
          (if (`KismetMathLibrary.InRange_FloatFloat` (+ (`KismetMathLibrary.FClamp` _relativerotation_pitch -70.0 80.0) AxisValue) -70.0 80.0 false false)
            (`SceneComponent.K2_AddRelativeRotation` _returnvalue (`KismetMathLibrary.MakeRotator` 0.0 AxisValue) false false)))))))

(event `self.ReceiveBeginPlay`
  (bind (_controllerset_leftcontroller _controllerset_rightcontroller) (break `/Game/AVRFramework/Structs/Struct_ControllerSet` (`/Game/AVRFramework/Blueprints/Components/Info/Comp_Controls.ControllerSet` (`self.Comp_Controller_VR`))))
  ;[1 1 1] Setup Pawn VR
  (`parent.ReceiveBeginPlay`)
  (set `self.PlayerSize` (`HeadMountedDisplayFunctionLibrary.GetWorldToMetersScale`))
  (`|ExecutionSequence`
    (:`then_0`
      (bind _gameinstance (`/Game/AVRFramework/Libraries/Lib_Core.getMainGameInstance` self))
      (bind _hmd (`/Game/AVRFramework/Blueprints/Game/BP_GameInstance_Main.getHMD` _gameinstance))
      (set `self.HMD` _hmd))
    (:`then_1`
      (`self.SetupHeight` (`self.PlayerHeight`))
      (if (`self.PausePawn`)
        (`self.SwitchControllers` "/Game/AVRFramework/Blueprints/VR/MotionControllers/BP_MotionController_Controller_Pause.BP_MotionController_Controller_Pause_C" "/Game/AVRFramework/Blueprints/VR/MotionControllers/BP_MotionController_Controller_Pause.BP_MotionController_Controller_Pause_C")
        (else
          (`self.SwitchControllers` _controllerset_leftcontroller _controllerset_rightcontroller)))
      (for _array_element (`|MakeArray` "NewEnumerator0" "NewEnumerator1" :!type "/Game/AVRFramework/Enums/Enum_Side Enum")
        (if (not (`HeadMountedDisplayFunctionLibrary.IsHeadMountedDisplayEnabled`))
          (`SceneComponent.K2_SetRelativeTransform` (select `/Game/AVRFramework/Enums/Enum_Side` _array_element :`NewEnumerator0` (`self.MotionControllerLeft`) :`NewEnumerator1` (`self.MotionControllerRight`)) (select `/Game/AVRFramework/Enums/Enum_Side` _array_element :`NewEnumerator0` (`SceneComponent.GetRelativeTransform` (`self.LeftSideArrow`)) :`NewEnumerator1` (`SceneComponent.GetRelativeTransform` (`self.RightSideArrow`))) false false))))))

(event `InputAction|MotionControllerTriggerRight`
  (params (Key :type "Key Structure"))
  ;[1 1 1] Forward Inputs to Motion Controller
  (:`Pressed`
    (goto _label :!via `RightPressed`))
  (:`Released`
    (goto _label :!via `RightReleased`)))

(event `InputAction|FaceButton01Right`
  (params (Key :type "Key Structure"))
  ;[1 1 1] Forward Inputs to Motion Controller
  (:`Pressed`
    (goto _label_2 :!via `RightPressed`))
  (:`Released`
    (goto _label_2 :!via `RightReleased`)))

(event `InputAxis|CapTouchPointingRight`
  (params (AxisValue :type "Float (single-precision)"))
  ;[1 1 1] Forward Inputs to Motion Controller
  (bind _controller (`self.GetController` "NewEnumerator1")
    (:`found`
      (`/Game/AVRFramework/Blueprints/VR/MotionControllers/BP_MotionController.TriggerCapTouch` _controller AxisValue))))

(event `InputAction|MotionControllerGripLeft`
  (params (Key :type "Key Structure"))
  ;[1 1 1] Forward Inputs to Motion Controller
  (:`Pressed`
    (`self.SetButtonSet` "NewEnumerator2" :!label _label_3))
  (:`Released`
    (goto _label_3 :!via `LeftReleased`)))

(event `InputAction|FaceButton02Left`
  (params (Key :type "Key Structure"))
  ;[1 1 1] Forward Inputs to Motion Controller
  (:`Pressed`
    (`self.SetButtonSet` "NewEnumerator4" :!label _label_4))
  (:`Released`
    (goto _label_4 :!via `LeftReleased`)))

(event `InputAxis|LookRight`
  (params (AxisValue :type "Float (single-precision)"))
  ;[1 1 1] Keyboard Inputs For Spectator
  (bind _spectator (`self.Spectator`)
    (:`then`
      (`/Game/AVRFramework/Blueprints/Pawn/BP_Pawn_NonVR.LookRight` _spectator AxisValue))
    (:`else`
      (`self.HasManualControl`
        (:`true`
          (`SceneComponent.K2_AddRelativeRotation` (`self.CurrentlyFocusedComponent`) (`KismetMathLibrary.MakeRotator` 0.0 0.0 AxisValue) false false))))))

(event `InputAxis|CapTouchThumbLeft`
  (params (AxisValue :type "Float (single-precision)"))
  ;[1 1 1] Forward Inputs to Motion Controller
  (bind _controller (`self.GetController` "NewEnumerator0")
    (:`found`
      (`/Game/AVRFramework/Blueprints/VR/MotionControllers/BP_MotionController.ThumbCapTouch` _controller AxisValue))))

(event `InputAction|MotionControllerGripRight`
  (params (Key :type "Key Structure"))
  ;[1 1 1] Forward Inputs to Motion Controller
  (:`Pressed`
    (goto _label_3 :!via `RightPressed`))
  (:`Released`
    (goto _label_3 :!via `RightReleased`)))

(event `InputAction|FaceButton02Right`
  (params (Key :type "Key Structure"))
  ;[1 1 1] Forward Inputs to Motion Controller
  (:`Pressed`
    (goto _label_4 :!via `RightPressed`))
  (:`Released`
    (goto _label_4 :!via `RightReleased`)))

(event `SetupHeight`
  (params (Height :type "Float (double-precision)" :default 180.0))
  ;[1 1 1] Setup Pawn VR
  ;;[1 1 1] Setup Hight and Tracking Origin
  (switch `/Game/AVRFramework/Enums/Enum_HMD` (`self.HMD`)
    (:`NewEnumerator3`
      (`HeadMountedDisplayFunctionLibrary.SetTrackingOrigin` "Floor" :!label _label_5))
    (:`NewEnumerator0`
      (goto _label_5))
    (:`NewEnumerator1`
      (goto _label_5))
    (:`NewEnumerator2`
      (`HeadMountedDisplayFunctionLibrary.SetTrackingOrigin` "Eye")
      (`SceneComponent.K2_AddLocalOffset` (`self.VRHandle`) (`KismetMathLibrary.MakeVector` 0.0 0.0 Height) false false))))

(event `InputAxis|CapTouchThumbRight`
  (params (AxisValue :type "Float (single-precision)"))
  ;[1 1 1] Forward Inputs to Motion Controller
  (bind _controller (`self.GetController` "NewEnumerator1")
    (:`found`
      (`/Game/AVRFramework/Blueprints/VR/MotionControllers/BP_MotionController.ThumbCapTouch` _controller AxisValue))))

(event `InputAction|ThumbstickPressLeft`
  (params (Key :type "Key Structure"))
  ;[1 1 1] Forward Inputs to Motion Controller
  (:`Pressed`
    (`self.SetButtonSet` "NewEnumerator7" :!label _label_6))
  (:`Released`
    (goto _label_6 :!via `LeftReleased`)))

(event `InputAction|FaceButton03Left`
  (params (Key :type "Key Structure"))
  ;[1 1 1] Forward Inputs to Motion Controller
  (:`Pressed`
    (`self.SetButtonSet` "NewEnumerator5" :!label _label_7))
  (:`Released`
    (goto _label_7 :!via `LeftReleased`)))

(event `InputAxis|Right`
  (params (AxisValue :type "Float (single-precision)"))
  (bind _returnvalue (`self.CurrentlyFocusedComponent`))
  ;[1 1 1] Keyboard Inputs For Spectator
  (bind _spectator (`self.Spectator`)
    (:`then`
      (`/Game/AVRFramework/Blueprints/Pawn/BP_Pawn_NonVR.MoveRight` _spectator AxisValue))
    (:`else`
      (`self.HasManualControl`
        (:`true`
          (`SceneComponent.K2_AddWorldOffset` _returnvalue (* (`SceneComponent.GetRightVector` _returnvalue) AxisValue) false false))))))

(event `InputAction|ThumbstickPressRight`
  (params (Key :type "Key Structure"))
  ;[1 1 1] Forward Inputs to Motion Controller
  (:`Pressed`
    (goto _label_6 :!via `RightPressed`))
  (:`Released`
    (goto _label_6 :!via `RightReleased`)))

(event `InputAxis|Grip1AxisLeft`
  (params (AxisValue :type "Float (single-precision)"))
  ;[1 1 1] Forward Inputs to Motion Controller
  (bind _controller (`self.GetController` "NewEnumerator0")
    (:`found`
      (`/Game/AVRFramework/Blueprints/VR/MotionControllers/BP_MotionController.GribAxis` _controller AxisValue))))

(event `InputAction|FaceButton03Right`
  (params (Key :type "Key Structure"))
  ;[1 1 1] Forward Inputs to Motion Controller
  (:`Pressed`
    (goto _label_7 :!via `RightPressed`))
  (:`Released`
    (goto _label_7 :!via `RightReleased`)))

(event `InputAction|ShoulderLeft`
  (params (Key :type "Key Structure"))
  ;[1 1 1] Forward Inputs to Motion Controller
  (:`Pressed`
    (`self.SetButtonSet` "NewEnumerator8" :!label _label_8))
  (:`Released`
    (goto _label_8 :!via `LeftReleased`)))

(event `InputAxis|Grip1AxisRight`
  (params (AxisValue :type "Float (single-precision)"))
  ;[1 1 1] Forward Inputs to Motion Controller
  (bind _controller (`self.GetController` "NewEnumerator1")
    (:`found`
      (`/Game/AVRFramework/Blueprints/VR/MotionControllers/BP_MotionController.GribAxis` _controller AxisValue))))

(event `InputAction|FaceButton04Left`
  (params (Key :type "Key Structure"))
  ;[1 1 1] Forward Inputs to Motion Controller
  (:`Pressed`
    (`self.SetButtonSet` "NewEnumerator6" :!label _label_9))
  (:`Released`
    (goto _label_9 :!via `LeftReleased`)))

(event `InputAxis|Forward`
  (params (AxisValue :type "Float (single-precision)"))
  (bind _returnvalue (`self.CurrentlyFocusedComponent`))
  ;[1 1 1] Keyboard Inputs For Spectator
  (bind _spectator (`self.Spectator`)
    (:`then`
      (`/Game/AVRFramework/Blueprints/Pawn/BP_Pawn_NonVR.MoveForward` _spectator AxisValue))
    (:`else`
      (`self.HasManualControl`
        (:`true`
          (`SceneComponent.K2_AddWorldOffset` _returnvalue (* (`SceneComponent.GetForwardVector` _returnvalue) AxisValue) false false))))))

(event `InputAction|ShoulderRight`
  (params (Key :type "Key Structure"))
  ;[1 1 1] Forward Inputs to Motion Controller
  (:`Pressed`
    (goto _label_8 :!via `RightPressed`))
  (:`Released`
    (goto _label_8 :!via `RightReleased`)))

(event `InputAxis|TriggerAxisLeft`
  (params (AxisValue :type "Float (single-precision)"))
  ;[1 1 1] Forward Inputs to Motion Controller
  (bind _controller (`self.GetController` "NewEnumerator0")
    (:`found`
      (`/Game/AVRFramework/Blueprints/VR/MotionControllers/BP_MotionController.TriggerAxis` _controller AxisValue))))

(event `self.SetPlayerSize`
  (params (Size :type "Float (single-precision)"))
  ;[1 1 1] Setup Pawn VR
  ;;[1 1 1] Set Player Size
  (`parent.SetPlayerSize` Size)
  (`HeadMountedDisplayFunctionLibrary.SetWorldToMetersScale` (`self.PlayerSize`)))

(event `InputAction|FaceButton04Right`
  (params (Key :type "Key Structure"))
  ;[1 1 1] Forward Inputs to Motion Controller
  (:`Pressed`
    (goto _label_9 :!via `RightPressed`))
  (:`Released`
    (goto _label_9 :!via `RightReleased`)))

(event `InputAxis|TriggerAxisRight`
  (params (AxisValue :type "Float (single-precision)"))
  ;[1 1 1] Forward Inputs to Motion Controller
  (bind _controller (`self.GetController` "NewEnumerator1")
    (:`found`
      (`/Game/AVRFramework/Blueprints/VR/MotionControllers/BP_MotionController.TriggerAxis` _controller AxisValue))))

(event `InputAxis|Up`
  (params (AxisValue :type "Float (single-precision)"))
  ;[1 1 1] Keyboard Inputs For Spectator
  (bind _spectator (`self.Spectator`)
    (:`then`
      (`/Game/AVRFramework/Blueprints/Pawn/BP_Pawn_NonVR.MoveUp` _spectator AxisValue))
    (:`else`)))

(event `SwitchControllers`
  (params (LeftController :type "/Game/AVRFramework/Blueprints/VR/MotionControllers/BP_MotionController Class Reference") (RightController :type "/Game/AVRFramework/Blueprints/VR/MotionControllers/BP_MotionController Class Reference"))
  ;[1 1 1] Setup Pawn VR
  ;;[1 1 1] Setup VR Controllers
  (`self.SetUpHand` LeftController)
  (`self.SetUpHand` RightController "NewEnumerator1")
  (`self.SetPlayerSize` (`self.PlayerSize`)))

(event `Key|SpaceBar`
  (params (Key :type "Key Structure"))
  ;[1 1 1] Keyboard Inputs For Spectator
  (:`Pressed`
    (bind _spectator (`self.Spectator`)
      (:`then`
        (`/Game/AVRFramework/Blueprints/Pawn/BP_Pawn_NonVR.SetJump` _spectator true))
      (:`else`
        (`self.HasManualControl`
          (:`true`
            (set `self.MoveFocus` (`/Game/AVRFramework/Libraries/FLib_Utility.IncrementIntWithModulo` (`self.MoveFocus`) 3)))))))
  (:`Released`
    (bind _spectator_2 (`self.Spectator`)
      (:`then`
        (`/Game/AVRFramework/Blueprints/Pawn/BP_Pawn_NonVR.SetJump` _spectator_2 false))
      (:`else`))))

(event `self.TeleportCharacter`
  (params (DestLocation :type "Vector Structure") (DestRotation :type "Rotator Structure") (WorldSize :type "Float (single-precision)") (TeleportTime :type "Float (single-precision)") (UseRotation :type Boolean) (UseMotion :type Boolean) (UseWorldSize :type Boolean) (UseFade :type Boolean))
  (`self.AdjustCorrectCapsuleLocation`)
  (`parent.TeleportCharacter` DestLocation DestRotation WorldSize TeleportTime UseRotation UseMotion UseWorldSize UseFade))

(event `self.ReceiveTick`
  (params (DeltaSeconds :type "Float (single-precision)"))
  (bind _returnvalue (`self.GetInputAxisValue`))
  (bind _returnvalue_2 (`self.GetInputAxisValue`))
  (bind _returnvalue_3 (`self.GetInputAxisValue`))
  (bind _returnvalue_4 (`self.GetInputAxisValue`))
  (bind _returnvalue_5 (`self.GetInputAxisValue`))
  (bind _returnvalue_6 (`self.GetInputAxisValue`))
  (bind _returnvalue_7 (* (`self.GetInputAxisValue`) -1.0))
  (bind _returnvalue_8 (* (`self.GetInputAxisValue`) -1.0))
  (bind (_relativelocation_x _relativelocation_y _relativelocation_z) (`KismetMathLibrary.BreakVector` (`SceneComponent.RelativeLocation` (`self.Camera`))))
  (bind _returnvalue_9 (/ _relativelocation_z 2.0))
  (bind (_outrotation _outrotationnooffset) (`self.CalculateRotation` _returnvalue_8 _returnvalue_6))
  (bind (_outrotation_2 _outrotationnooffset_2) (`self.CalculateRotation` _returnvalue_7 _returnvalue_5))
  (bind _returnvalue_10 (- (`CapsuleComponent.GetUnscaledCapsuleHalfHeight` (`self.CapsuleComponent`)) _returnvalue_9))
  (`parent.ReceiveTick` DeltaSeconds)
  (`|ExecutionSequence`
    (:`then_0`
      (bind _controller (`self.GetController` "NewEnumerator0")
        (:`found`
          (`/Game/AVRFramework/Blueprints/VR/MotionControllers/BP_MotionController.SetThumbstickRotation` _controller _outrotation_2 _outrotationnooffset_2 _returnvalue_7 _returnvalue_5))))
    (:`then_1`
      (bind _controller_2 (`self.GetController` "NewEnumerator1")
        (:`found`
          (`/Game/AVRFramework/Blueprints/VR/MotionControllers/BP_MotionController.SetThumbstickRotation` _controller_2 _outrotation _outrotationnooffset _returnvalue_8 _returnvalue_6))))
    (:`then_2`
      (`|ExecutionSequence`
        (:`then_0`
          (`self.ThumbstickDirectionPressed` "NewEnumerator10" (> _returnvalue 0.6) (> _returnvalue_3 0.6)))
        (:`then_1`
          (`self.ThumbstickDirectionPressed` "NewEnumerator9" (< _returnvalue -0.6) (< _returnvalue_3 -0.6)))
        (:`then_2`
          (`self.ThumbstickDirectionPressed` "NewEnumerator12" (> _returnvalue_2 0.6) (> _returnvalue_4 0.6)))
        (:`then_3`
          (`self.ThumbstickDirectionPressed` "NewEnumerator11" (< _returnvalue_2 -0.6) (< _returnvalue_4 -0.6)))
        (:`then_4`
          (if (>= (`KismetMathLibrary.Abs` _returnvalue_10) 15.0)
            (bind _out (`/Game/AVRFramework/Libraries/FLib_Utility.SaveFloat` _returnvalue_10))
            (`CapsuleComponent.SetCapsuleHalfHeight` (`self.CapsuleComponent`) _returnvalue_9 true)
            (`self.K2_AddActorWorldOffset` (`KismetMathLibrary.MakeVector` 0.0 0.0 (* _out -1.0)))
            (`SceneComponent.K2_AddRelativeLocation` (`self.VRHandle`) (`KismetMathLibrary.MakeVector` 0.0 0.0 _out) false false)))))))

(event `AdjustCorrectCapsuleLocation`
  (bind (_returnvalue_x _returnvalue_y) (`KismetMathLibrary.BreakVector` (`self.K2_GetActorLocation`)))
  (bind (_returnvalue_x_2 _returnvalue_y_2 _returnvalue_z) (`KismetMathLibrary.BreakVector` (`self.K2_GetActorLocation`)))
  (bind (_returnvalue_x_3 _returnvalue_y_3) (`KismetMathLibrary.BreakVector` (`SceneComponent.K2_GetComponentLocation` (`self.Camera`))))
  (bind (_returnvalue_x_4 _returnvalue_y_4) (`KismetMathLibrary.BreakVector` (`SceneComponent.K2_GetComponentLocation` (`self.Camera`))))
  (if (`self.IsLocallyControlled`)
    (`self.LocallyControlled`
      (:`True`
        (bind _out (`/Game/AVRFramework/Libraries/FLib_Utility.SaveVector2D` (- (`KismetMathLibrary.MakeVector2D` _returnvalue_x_3 _returnvalue_y_3) (`KismetMathLibrary.MakeVector2D` _returnvalue_x _returnvalue_y))))
        (`self.K2_SetActorLocation` (`KismetMathLibrary.MakeVector` _returnvalue_x_4 _returnvalue_y_4 _returnvalue_z))
        (bind (_x _y) (`KismetMathLibrary.BreakVector2D` (* _out -1.0)))
        (`SceneComponent.K2_AddWorldOffset` (`self.VRHandle`) (`KismetMathLibrary.MakeVector` _x _y) false false))
      (:`False`))))

(event `Key|RightMouseButton`
  (params (Key :type "Key Structure"))
  ;[1 1 1] Keyboard Inputs For Spectator
  (:`Pressed`
    (bind _spectator (`self.Spectator`)
      (:`then`
        (`/Game/AVRFramework/Blueprints/Pawn/BP_Pawn_NonVR.ToggleMouse` _spectator))
      (:`else`
        (`self.HasManualControl`
          (:`true`
            (`self.ButtonFunctionality` "NewEnumerator2" :!label _label_10))))))
  (:`Released`
    (`self.Spectator`
      (:`then`)
      (:`else`
        (`self.HasManualControl`
          (:`true`
            (goto _label_10 :!via `Release`)))))))

(event `self.ReceivePossessed`
  (params (NewController :type "Controller Object Reference"))
  (`parent.ReceivePossessed` NewController)
  (bind _asbp_player_controller_main (cast `/Game/AVRFramework/Blueprints/Game/BP_PlayerController_Main` NewController))
  (`self.Client_InitializePawn` _asbp_player_controller_main))

(event `RotateThroughControllers`
  (bind _array (`|MakeArray` "/Game/AVRFramework/Blueprints/VR/MotionControllers/BP_MotionController_Controller_Laser.BP_MotionController_Controller_Laser_C" "/Game/AVRFramework/Blueprints/VR/MotionControllers/BP_MotionController_Controller_Laser_Single.BP_MotionController_Controller_Laser_Single_C" "/Game/AVRFramework/Blueprints/VR/MotionControllers/BP_MotionController_Hands.BP_MotionController_Hands_C" "/Game/AVRFramework/Blueprints/VR/MotionControllers/BP_MotionController_HandWithWatch.BP_MotionController_HandWithWatch_C" :!type "/Game/AVRFramework/Blueprints/VR/MotionControllers/BP_MotionController Class Reference"))
  ;[1 1 1] Switch between Controller Modi
  (bind _controller (`self.GetController` "NewEnumerator0")
    (:`found`
      (bind _output (`|GetArrayItem` _array (`/Game/AVRFramework/Libraries/FLib_Utility.IncrementIntWithModulo` (`KismetArrayLibrary.Array_Find` _array (`GameplayStatics.GetObjectClass` _controller)) (`KismetArrayLibrary.Array_Length` _array))))
      (`self.SwitchControllers` _output _output))))

(event `self.ReceiveUnpossessed`
  (params (OldController :type "Controller Object Reference"))
  (`parent.ReceiveUnpossessed` OldController)
  (`self.Client_DeinitializePawn`))

(event `Key|LeftMouseButton`
  (params (Key :type "Key Structure"))
  ;[1 1 1] Keyboard Inputs For Spectator
  (:`Pressed`
    (bind _spectator (`self.Spectator`)
      (:`then`
        (`/Game/AVRFramework/Blueprints/Pawn/BP_Pawn_NonVR.Trigger` _spectator true))
      (:`else`
        (`self.HasManualControl`
          (:`true`
            (`self.ButtonFunctionality` "NewEnumerator0" :!label _label_11))))))
  (:`Released`
    (bind _spectator_2 (`self.Spectator`)
      (:`then`
        (`/Game/AVRFramework/Blueprints/Pawn/BP_Pawn_NonVR.Trigger` _spectator_2 false))
      (:`else`
        (`self.HasManualControl`
          (:`true`
            (goto _label_11 :!via `Release`)))))))

(event `PawnReady_Event_0`
  (remove `/Game/AVRFramework/Blueprints/Game/BP_PlayerController_Main.PawnReady` (`self.MainPlayerController`) (delegate `PawnReady_Event_0`))
  (`BlueprintSetLibrary.Set_RemoveItems` (`/Game/AVRFramework/Blueprints/Components/Info/Comp_Controls.BlockedFunction` (`self.Comp_Controller_VR`)) (`|MakeArray` "NewEnumerator11" "NewEnumerator3" "NewEnumerator4" "NewEnumerator5" "NewEnumerator6" "NewEnumerator9" "NewEnumerator10" :!type "/Game/AVRFramework/Enums/Enum_Control_Function Enum")))

(event `self.Client_InitializePawn`
  (params (PlayerController :type "/Game/AVRFramework/Blueprints/Game/BP_PlayerController_Main Object Reference"))
  (`parent.Client_InitializePawn` PlayerController)
  (add `/Game/AVRFramework/Blueprints/Game/BP_PlayerController_Main.PawnReady` PlayerController (delegate `PawnReady_Event_0`))
  (`BlueprintSetLibrary.Set_AddItems` (`/Game/AVRFramework/Blueprints/Components/Info/Comp_Controls.BlockedFunction` (`self.Comp_Controller_VR`)) (`|MakeArray` "NewEnumerator11" "NewEnumerator3" "NewEnumerator4" "NewEnumerator5" "NewEnumerator6" "NewEnumerator9" "NewEnumerator10" :!type "/Game/AVRFramework/Enums/Enum_Control_Function Enum")))

(event `Key|E`
  (params (Key :type "Key Structure"))
  ;[1 1 1] Keyboard Inputs For Spectator
  (:`Pressed`
    (`self.HasManualControl`
      (:`true`
        (`self.ButtonFunctionality` "NewEnumerator3" :!label _label_12))))
  (:`Released`
    (`self.HasManualControl`
      (:`true`
        (goto _label_12 :!via `Release`)))))

(event `InputAction|Sprint`
  (params (Key :type "Key Structure"))
  ;[1 1 1] Keyboard Inputs For Spectator
  (:`Pressed`
    (bind _spectator (`self.Spectator`)
      (:`then`
        (`/Game/AVRFramework/Blueprints/Pawn/BP_Pawn_NonVR.SetSprint` _spectator true))
      (:`else`)))
  (:`Released`
    (bind _spectator_2 (`self.Spectator`)
      (:`then`
        (`/Game/AVRFramework/Blueprints/Pawn/BP_Pawn_NonVR.SetSprint` _spectator_2 false))
      (:`else`))))

(event `Key|Q`
  (params (Key :type "Key Structure"))
  ;[1 1 1] Keyboard Inputs For Spectator
  (:`Pressed`
    (`self.HasManualControl`
      (:`true`
        (`self.ButtonFunctionality` "NewEnumerator4" :!label _label_13))))
  (:`Released`
    (`self.HasManualControl`
      (:`true`
        (goto _label_13 :!via `Release`)))))

(event `InputAxis|Zoom`
  (params (AxisValue :type "Float (single-precision)"))
  ;[1 1 1] Keyboard Inputs For Spectator
  (bind _spectator (`self.Spectator`)
    (:`then`
      (`/Game/AVRFramework/Blueprints/Pawn/BP_Pawn_NonVR.Zoom` _spectator AxisValue))
    (:`else`)))

(event `Key|One`
  (params (Key :type "Key Structure"))
  ;[1 1 1] Spectator Mode, Still in Development
  (:`Pressed`
    (`self.SetSpectatorMode` 1)))

(event `Key|NumPadZero`
  (params (Key :type "Key Structure"))
  ;[1 1 1] Spectator Mode, Still in Development
  (:`Pressed`
    (`self.MoveSpectatorToPositionWithIndex` 0)))

(event `Key|Two`
  (params (Key :type "Key Structure"))
  ;[1 1 1] Spectator Mode, Still in Development
  (:`Pressed`
    (`self.SetSpectatorMode` 2)))

(event `Key|NumPadOne`
  (params (Key :type "Key Structure"))
  ;[1 1 1] Spectator Mode, Still in Development
  (:`Pressed`
    (`self.MoveSpectatorToPositionWithIndex` 1)))

(event `Key|Three`
  (params (Key :type "Key Structure"))
  ;[1 1 1] Spectator Mode, Still in Development
  (:`Pressed`
    (`self.SetSpectatorMode` 3)))

(event `Key|NumPadTwo`
  (params (Key :type "Key Structure"))
  ;[1 1 1] Spectator Mode, Still in Development
  (:`Pressed`
    (`self.MoveSpectatorToPositionWithIndex` 2)))

(event `Key|Four`
  (params (Key :type "Key Structure"))
  ;[1 1 1] Spectator Mode, Still in Development
  (:`Pressed`
    (`self.SetSpectatorMode` 4)))

(event `Key|NumPadThree`
  (params (Key :type "Key Structure"))
  ;[1 1 1] Spectator Mode, Still in Development
  (:`Pressed`
    (`self.MoveSpectatorToPositionWithIndex` 3)))

(event `SpawnSpectator`
  (params (Pawn :type "/Game/AVRFramework/Blueprints/Pawn/BP_Pawn_NonVR_Spectator Class Reference") (SpawnTransform :type "Transform Structure"))
  ;[1 1 1] Spectator Mode, Still in Development
  (bind _returnvalue (`|SpawnActorFromClass` Pawn SpawnTransform "AlwaysSpawn" "OverrideRootScale" self 30.0 (1920.0 1080.0) false null))
  (bind _output_get (set `self.Spectator` _returnvalue))
  (bind _asbp_player_controller_main (cast `/Game/AVRFramework/Blueprints/Game/BP_PlayerController_Main` (`self.GetController`)))
  (`self.Client_InitializePawn` _output_get _asbp_player_controller_main))

(event `Key|NumPadFour`
  (params (Key :type "Key Structure"))
  ;[1 1 1] Spectator Mode, Still in Development
  (:`Pressed`
    (`self.MoveSpectatorToPositionWithIndex` 4)))

(event `Key|NumPadFive`
  (params (Key :type "Key Structure"))
  ;[1 1 1] Spectator Mode, Still in Development
  (:`Pressed`
    (`self.MoveSpectatorToPositionWithIndex` 5)))

(event `Key|NumPadSix`
  (params (Key :type "Key Structure"))
  ;[1 1 1] Spectator Mode, Still in Development
  (:`Pressed`
    (`self.MoveSpectatorToPositionWithIndex` 6)))

(event `SetSpectatorMode`
  (params (Mode :type Integer))
  ;[1 1 1] Spectator Mode, Still in Development
  (switch `int` Mode
    (:`1`
      (`/Game/AVRFramework/Libraries/FLib_Utility.DeleteActor` (`self.Spectator`))
      (`HeadMountedDisplayFunctionLibrary.SetSpectatorScreenMode` "SingleEyeCroppedToFill"))
    (:`2`
      (`HeadMountedDisplayFunctionLibrary.SetSpectatorScreenMode` "Texture")
      (`/Engine/EditorBlueprintResources/StandardMacros.IsValid` (`self.Spectator`) :!label _label_14
        (:`Is Not Valid`
          (bind _spectatorposition (`self.GetBestSpectatorPosition`))
          (`/Engine/EditorBlueprintResources/StandardMacros.IsValid` _spectatorposition
            (:`Is Valid`
              (`self.SpawnSpectator` (`/Game/AVRFramework/Blueprints/Info/BP_Info_Level.Pawn_Spectator` (`/Game/AVRFramework/Libraries/Lib_Core.getInfoLevels` self)) (`self.GetTransform` _spectatorposition)))))))
    (:`3`
      (`HeadMountedDisplayFunctionLibrary.SetSpectatorScreenMode` "TexturePlusEye")
      (`HeadMountedDisplayFunctionLibrary.SetSpectatorScreenModeTexturePlusEyeLayout` (0.7 0.02) (0.98 0.4) (0.0 0.0) (1.0 1.0) false)
      (goto _label_14))
    (:`4`
      (`HeadMountedDisplayFunctionLibrary.SetSpectatorScreenMode` "TexturePlusEye")
      (`HeadMountedDisplayFunctionLibrary.SetSpectatorScreenModeTexturePlusEyeLayout` (0.0 0.0) (1.0 1.0) (0.7 0.02) (0.98 0.4))
      (goto _label_14))))

(event `Key|NumPadSeven`
  (params (Key :type "Key Structure"))
  ;[1 1 1] Spectator Mode, Still in Development
  (:`Pressed`
    (`self.MoveSpectatorToPositionWithIndex` 7)))

(event `Key|NumPadEight`
  (params (Key :type "Key Structure"))
  ;[1 1 1] Spectator Mode, Still in Development
  (:`Pressed`
    (`self.MoveSpectatorToPositionWithIndex` 8)))

(event `Key|NumPadNine`
  (params (Key :type "Key Structure"))
  ;[1 1 1] Spectator Mode, Still in Development
  (:`Pressed`
    (`self.MoveSpectatorToPositionWithIndex` 9)))

(fn `CalculateRotation`
  (params (Up :type "Float (double-precision)") (Right :type "Float (double-precision)"))
  (returns (OutRotation :type "Rotator Structure") (OutRotationNoOffset :type "Rotator Structure"))
  (bind _returnvalue (`KismetMathLibrary.Normal` (`KismetMathLibrary.MakeVector` Up Right)))
  (return (`KismetMathLibrary.Conv_VectorToRotator` (`KismetMathLibrary.GreaterGreater_VectorRotator` _returnvalue (`KismetMathLibrary.MakeRotator` 0.0 0.0 (.yaw (`self.K2_GetActorRotation`))))) (`KismetMathLibrary.Conv_VectorToRotator` _returnvalue)))

(fn `GetBestSpectatorPosition`
  (returns (SpectatorPosition :type "/Game/AVRFramework/Blueprints/Navigation/BP_SpectatorPosition Object Reference"))
  (locals (DefaultSpectator :type "/Game/AVRFramework/Blueprints/Navigation/BP_SpectatorPosition Object Reference"))
  (bind _outactors (`GameplayStatics.GetAllActorsOfClass` "/Game/AVRFramework/Blueprints/Navigation/BP_SpectatorPosition.BP_SpectatorPosition_C"))
  (for _array_element _outactors
    (if (== (`/Game/AVRFramework/Blueprints/Navigation/BP_SpectatorPosition.Index` _array_element) 1)
      (return _array_element)
      (elif (`/Game/AVRFramework/Blueprints/Navigation/BP_SpectatorPosition.DefaultSpectatorPosition` _array_element)
        (set `local.DefaultSpectator` _array_element))))
  (return (`local.DefaultSpectator`)))

(fn `GetCameraComponent`
  (returns (Camera :type "CameraComponent Object Reference"))
  (return (`self.Camera`)))

(fn `GetSpectatorPositionFromIndex`
  (params (Index :type Integer))
  (returns (SpectatorPosition :type "/Game/AVRFramework/Blueprints/Navigation/BP_SpectatorPosition Object Reference"))
  (locals (DefaultSpectator :type "/Game/AVRFramework/Blueprints/Navigation/BP_SpectatorPosition Object Reference"))
  (bind _outactors (`GameplayStatics.GetAllActorsOfClass` "/Game/AVRFramework/Blueprints/Navigation/BP_SpectatorPosition.BP_SpectatorPosition_C"))
  (for _array_element _outactors
    (if (== (`/Game/AVRFramework/Blueprints/Navigation/BP_SpectatorPosition.Index` _array_element) Index)
      (return _array_element)))
  (`/Game/AVRFramework/Libraries/Lib_Core.ErrorMessage` self "NewEnumerator0" self "Spectator Position Not Found")
  (return null))

(fn `GetWorldScaleFactor`
  (returns (`Out ScaleFactor` :type "Float (double-precision)"))
  (return (/ (`HeadMountedDisplayFunctionLibrary.GetWorldToMetersScale`) 100.0)))

(fn `SetUpHand`
  (params (MotionControllerClass :type "/Game/AVRFramework/Blueprints/VR/MotionControllers/BP_MotionController Class Reference") (Side :type "/Game/AVRFramework/Enums/Enum_Side Enum" :default "NewEnumerator0"))
  (bind _controller (`self.GetController` Side)
    (:`found`
      (`/Game/AVRFramework/Libraries/FLib_Utility.DeleteActor` _controller))
    (:`NotFound`
      _))
  (`|SpawnActorFromClass` (select `bool` (`KismetSystemLibrary.IsValidClass` MotionControllerClass) :`false` "/Game/AVRFramework/Blueprints/VR/MotionControllers/BP_MotionController_Controller_Pause.BP_MotionController_Controller_Pause_C" :`true` MotionControllerClass) (`KismetMathLibrary.MakeTransform` (0.0 0.0 0.0)) "AlwaysSpawn" "OverrideRootScale" self self (`self.HMD`) Side (select `/Game/AVRFramework/Enums/Enum_Side` Side :`NewEnumerator0` (`self.MotionControllerLeft`) :`NewEnumerator1` (`self.MotionControllerRight`)) self))

(fn `UserConstructionScript`)