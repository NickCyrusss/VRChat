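; Motion controller Blueprint variant that keeps the VR controller mesh ticking while the game is paused.
; On BeginPlay it makes the controller mesh component tickable when paused, then runs SetupControllerMesh.
; That function looks up one entry in the component map and applies the same flag to it and to the timeline components it returns.
; SetMeshVisibility shows or hides that mapped component, mostly when taking a tool.
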(event `self.ReceiveTick`
  (params (DeltaSeconds :type "Float (single-precision)"))
  (`parent.ReceiveTick` DeltaSeconds))

(event `self.ReceiveBeginPlay`
  (bind (_value _returnvalue) (`BlueprintMapLibrary.Map_Find` (`self.MCompMap`) "NewEnumerator0"))
  ;[1 1 1] Setup
  (`parent.ReceiveBeginPlay`)
  (`ActorComponent.SetTickableWhenPaused` (`self.ControllerMeshComponent`) true)
  (if _returnvalue
    (`self.SetTickableWhenPaused` _value true)
    (for _array_element (`self.K2_GetComponentsByClass` _value "/Script/Engine.TimelineComponent")
      (`ActorComponent.SetTickableWhenPaused` _array_element true))))

(event `self.SetMeshVisibility`
  (params (Set :type Boolean))
  ;[1 1 1] Set Visiblity mostly when taking Tool
  (`/Game/AVRFramework/Blueprints/VR/MotionComponents/BP_MComp.SetVisibility` (`BlueprintMapLibrary.Map_Find` (`self.MCompMap`) "NewEnumerator0") Set))

(fn `UserConstructionScript`
  (`parent.UserConstructionScript`))