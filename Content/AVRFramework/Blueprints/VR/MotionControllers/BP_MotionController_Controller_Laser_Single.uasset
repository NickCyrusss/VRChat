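; Laser motion controller variant for the AVR framework that limits which hand shows its laser, favouring the right.
; It overrides ShouldLaserBeActive: when the parent check passes, the right controller's laser is always active.
; The left laser activates only while the right controller grabs an actor whose Comp_Grab has SnapAndReplaceControls set, found through the VR pawn's controller and component maps.
; BeginPlay, Tick and construction just call the parent.
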(event `self.ReceiveBeginPlay`
  (`parent.ReceiveBeginPlay`))

(event `self.ReceiveTick`
  (params (DeltaSeconds :type "Float (single-precision)"))
  (`parent.ReceiveTick` DeltaSeconds))

(fn `ShouldLaserBeActive`
  (returns (ShouldBeActive :type Boolean))
  (bind _value (`BlueprintMapLibrary.Map_Find` (`/Game/AVRFramework/Blueprints/Pawn/BP_Pawn_VR.Controllers` (`self.VRPawn`)) "NewEnumerator1"))
  (bind (_value_2 _returnvalue) (`BlueprintMapLibrary.Map_Find` (`/Game/AVRFramework/Blueprints/VR/MotionControllers/BP_MotionController.MCompMap` _value) "NewEnumerator2"))
  (if (`parent.ShouldLaserBeActive`)
    (switch `/Game/AVRFramework/Enums/Enum_Side` (`self.Side`)
      (:`NewEnumerator0`
        (`/Engine/EditorBlueprintResources/StandardMacros.IsValid` _value
          (:`Is Valid`
            (if _returnvalue
              (`/Engine/EditorBlueprintResources/StandardMacros.IsValid` _value_2
                (:`Is Valid`
                  (bind _grabbedactor (message `/Game/AVRFramework/Interface/Interface_GrabbingActor.GrabbingActor_getCurrentlyGrabbedActor` _value_2))
                  (`/Engine/EditorBlueprintResources/StandardMacros.IsValid` _grabbedactor
                    (:`Is Valid`
                      (bind _returnvalue_2 (`self.GetComponentByClass` _grabbedactor "/Game/AVRFramework/Blueprints/Components/Interaction/Comp_Grab.Comp_Grab_C"))
                      (`/Engine/EditorBlueprintResources/StandardMacros.IsValid` _returnvalue_2
                        (:`Is Valid`
                          (return (`/Game/AVRFramework/Blueprints/Components/Interaction/Comp_Grab.SnapAndReplaceControls` _returnvalue_2)))
                        (:`Is Not Valid`
                          _)))
                    (:`Is Not Valid`
                      _))
                  (return false))
                (:`Is Not Valid`
                  _))))
          (:`Is Not Valid`
            _))
        (return false))
      (:`NewEnumerator1`
        (return true)))
    (else
      (return false))))

(fn `UserConstructionScript`
  (`parent.UserConstructionScript`))