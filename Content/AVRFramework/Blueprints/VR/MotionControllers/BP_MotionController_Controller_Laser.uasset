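; VR motion controller Blueprint with a laser pointer that switches off while certain other controller components, per its comment the radial menu or teleporter, are active.
; Each tick with a valid VR pawn, it derives the laser's desired state from those components in MCompMap, an enum-keyed component map.
; An OnlyIfDifferent gate limits activation calls to state changes.
; SetMeshVisibility shows or hides the laser and another mapped component, mostly when taking a tool.
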(event `self.ReceiveTick`
  (params (DeltaSeconds :type "Float (single-precision)"))
  (bind _shouldbeactive (`self.ShouldLaserBeActive`))
  (bind _value (`BlueprintMapLibrary.Map_Find` (`self.MCompMap`) "NewEnumerator2"))
  (bind (_value_2 _returnvalue) (`BlueprintMapLibrary.Map_Find` (`self.MCompMap`) "NewEnumerator2"))
  ;[1 1 1] Activate/Deactivate Laserpointer when opening Radial Menu or starting Teleporter
  (`parent.ReceiveTick` DeltaSeconds)
  (`/Engine/EditorBlueprintResources/StandardMacros.IsValid` (`self.VRPawn`)
    (:`Is Valid`
      (if _returnvalue
        (if (!= (`/Game/AVRFramework/Blueprints/VR/MotionComponents/BP_MComp.Active` _value_2) _shouldbeactive)
          (if _shouldbeactive
            (`/Game/AVRFramework/Blueprints/VR/MotionComponents/BP_MComp.MCompSetActive` _value true)
            (else
              (`/Game/AVRFramework/Blueprints/VR/MotionComponents/BP_MComp.MCompSetActive` _value false))))))))

(event `self.SetMeshVisibility`
  (params (Set :type Boolean))
  ;[1 1 1] Set Visiblity mostly when taking Tool
  (`/Game/AVRFramework/Blueprints/VR/MotionComponents/BP_MComp.SetVisibility` (`BlueprintMapLibrary.Map_Find` (`self.MCompMap`) "NewEnumerator2") Set)
  (`/Game/AVRFramework/Blueprints/VR/MotionComponents/BP_MComp.SetVisibility` (`BlueprintMapLibrary.Map_Find` (`self.MCompMap`) "NewEnumerator0") Set))

(fn `ShouldLaserBeActive`
  (returns (ShouldBeActive :type Boolean))
  (bind _mcompmap (`self.MCompMap`))
  (bind (_value _returnvalue) (`BlueprintMapLibrary.Map_Find` _mcompmap "NewEnumerator7"))
  (bind (_value_2 _returnvalue_2) (`BlueprintMapLibrary.Map_Find` _mcompmap "NewEnumerator5"))
  (if _returnvalue_2
    (if (not (`/Game/AVRFramework/Blueprints/VR/MotionComponents/BP_MComp.Active` _value_2))
      (if _returnvalue :!label _label
        (if (`/Game/AVRFramework/Blueprints/VR/MotionComponents/BP_MComp.Active` _value)
          _
          (else
            (return true)))
        (else
          (return true))))
    (else
      (goto _label)))
  (return false))

(fn `UserConstructionScript`
  (`parent.UserConstructionScript`))