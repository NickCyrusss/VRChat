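; VR motion controller actor for one hand, which registers with the VR pawn and attaches to its motion controller component.
; It maps child-actor MComp modules and routes key input to them through the pawn's key mapping, honoring blocked functions and a prioritized MComp, which two functions bypass.
; It also stores thumbstick, trigger, grip and touch values, forwards highlights and color to the controller MComp, and plays timeline-shaped haptics through the player controller.
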(event `self.ReceiveTick`
  (params (DeltaSeconds :type "Float (single-precision)")))

(event `self.ReceiveBeginPlay`
  (bind _vrpawn (`self.VRPawn`))
  (bind _motioncontrollercomponent (`self.MotionControllerComponent`))
  ;[1 1 1] Setup
  (`parent.ReceiveBeginPlay`)
  (`/Game/AVRFramework/Libraries/MLib_Actor_Macros.WaitForObjectToValidate` _vrpawn
    (:`Is Valid`
      (`/Game/AVRFramework/Blueprints/Pawn/BP_Pawn_Base.RegisterActorToPawn` _vrpawn self true)
      (`BlueprintMapLibrary.Map_Add` (`/Game/AVRFramework/Blueprints/Pawn/BP_Pawn_VR.Controllers` _vrpawn) (`self.Side`) self)
      (`/Game/AVRFramework/Libraries/MLib_Actor_Macros.WaitForObjectToValidate` _motioncontrollercomponent
        (:`Is Valid`
          (`self.K2_AttachToComponent` _motioncontrollercomponent "None" "KeepRelative" "KeepRelative" "KeepRelative" false)
          (`self.UpdateMCompMap`))))))

(event `KeyInput`
  (params (Set :type Boolean) (Key :type "/Game/AVRFramework/Enums/Enum_Controller_Buttons Enum" :default "NewEnumerator1"))
  (bind _prioritisedmcomp (`self.PrioritisedMComp`))
  (bind (_value _returnvalue) (`BlueprintMapLibrary.Map_Find` (`/Game/AVRFramework/Blueprints/Components/Info/Comp_Controls.getKeyMapping` (`/Game/AVRFramework/Blueprints/Pawn/BP_Pawn_VR.Comp_Controller_VR` (`self.VRPawn`))) (`self.Side`)))
  (bind (_value_2 _returnvalue_2) (`BlueprintMapLibrary.Map_Find` (break `/Game/AVRFramework/Structs/Struct_KeyToFunctionMap` _value) Key))
  ;[1 1 1] Assign Button Actions
  (bind _asbp_mcomp_controller (`self.GetControllerMComp`)
    (:`then`
      (`/Game/AVRFramework/Blueprints/VR/MotionComponents/BP_MComp_Controller.SetButtonHighlight` _asbp_mcomp_controller Key Set))
    (:`CastFailed`
      _))
  (`/Engine/EditorBlueprintResources/StandardMacros.IsValid` (`self.PrioritisedMComp`)
    (:`Is Valid`
      (`/Game/AVRFramework/Blueprints/VR/MotionComponents/BP_MComp.KeyPressed` (`self.PrioritisedMComp`) Key Set))
    (:`Is Not Valid`
      _))
  (if _returnvalue
    (if _returnvalue_2
      (if (not (`BlueprintSetLibrary.Set_Contains` (`/Game/AVRFramework/Blueprints/Components/Info/Comp_Controls.BlockedFunction` (`/Game/AVRFramework/Blueprints/Pawn/BP_Pawn_VR.Comp_Controller_VR` (`self.VRPawn`))) _value_2))
        (bind _keys (`BlueprintMapLibrary.Map_Keys` (`self.MCompMap`)))
        (for _array_element _keys
          (bind (_value_3 _returnvalue_3) (`BlueprintMapLibrary.Map_Find` (`self.MCompMap`) _array_element))
          (if _returnvalue_3
            (if (or (`|EnumEquality` _value_2 "NewEnumerator2") (`|EnumEquality` _value_2 "NewEnumerator3"))
              (`/Game/AVRFramework/Blueprints/VR/MotionComponents/BP_MComp.FunctionInput` _value_3 _value_2 Set :!label _label)
              (else
                (`/Engine/EditorBlueprintResources/StandardMacros.IsValid` _prioritisedmcomp
                  (:`Is Valid`
                    (if (== _prioritisedmcomp _value_3)
                      (goto _label)))
                  (:`Is Not Valid`
                    (goto _label)))))))))))

(event `SetReplacedControls`
  (params (Set :type Boolean) (PriorityMComp :type "/Game/AVRFramework/Blueprints/VR/MotionComponents/BP_MComp Object Reference"))
  ;[1 1 1] Assign Button Actions
  (if Set
    (set `self.PrioritisedMComp` PriorityMComp)
    (else
      (set `self.PrioritisedMComp` null))))

(event `UpdateMCompMap`
  ;[1 1 1] Create MComp Map
  (`BlueprintMapLibrary.Map_Clear` (`self.MCompMap`))
  (for _array_element (`self.K2_GetComponentsByClass` "/Script/Engine.ChildActorComponent")
    (bind _asbp_mcomp (cast `/Game/AVRFramework/Blueprints/VR/MotionComponents/BP_MComp` (`ChildActorComponent.ChildActor` _array_element)))
    (`BlueprintMapLibrary.Map_Add` (`self.MCompMap`) (`/Game/AVRFramework/Blueprints/VR/MotionComponents/BP_MComp.MComp` _asbp_mcomp) _asbp_mcomp)))

(event `DesiredControllerColor`
  (params (DesiredColor :type "LinearColor Structure"))
  ;[1 1 1] AdjustVisuals
  (bind _asbp_mcomp_controller (`self.GetControllerMComp`)
    (:`then`
      (`/Game/AVRFramework/Blueprints/VR/MotionComponents/BP_MComp_Controller.SetTrimColor` _asbp_mcomp_controller DesiredColor))))

(event `SetHaptics`
  (params (Curve :type "/Game/AVRFramework/Enums/Enum_Haptic_Curves Enum" :default "NewEnumerator4") (Duration :type "Float (double-precision)") (Strength :type "Float (double-precision)"))
  (bind _returnvalue (/ 1.0 Duration))
  ;[1 1 1] Haptics
  (`self.LocallyControlled`)
  (if (== Duration 0.0)
    (`self.ExecuteHaptic` 0.01 1.0 Strength :!label _label_2)
    (else
      (switch `/Game/AVRFramework/Enums/Enum_Haptic_Curves` Curve
        (:`NewEnumerator4`
          (goto _label_2))
        (:`NewEnumerator0`
          (`TimelineComponent.SetPlayRate` (`self.HapticsTimelineConstant`) _returnvalue)
          (bind (_direction _percent) (`Timeline|HapticsTimelineConstant` :!via `PlayFromStart`)
            (:`Update`
              (`self.ExecuteHaptic` 0.01 _percent Strength))))
        (:`NewEnumerator1`
          (`TimelineComponent.SetPlayRate` (`self.HapticsTimelineUpCurve`) _returnvalue)
          (bind (_direction_2 _percent_2) (`Timeline|HapticsTimelineUpCurve` :!via `PlayFromStart`)
            (:`Update`
              (`self.ExecuteHaptic` 0.01 _percent_2 Strength))))
        (:`NewEnumerator2`
          (`TimelineComponent.SetPlayRate` (`self.HapticsTimelineDownCurve`) _returnvalue)
          (bind (_direction_3 _percent_3) (`Timeline|HapticsTimelineDownCurve` :!via `PlayFromStart`)
            (:`Update`
              (`self.ExecuteHaptic` 0.01 _percent_3 Strength))))
        (:`NewEnumerator3`
          (`TimelineComponent.SetPlayRate` (`self.HapticsTimelineNormalCurve`) _returnvalue)
          (bind (_direction_4 _percent_4) (`Timeline|HapticsTimelineNormalCurve` :!via `PlayFromStart`)
            (:`Update`
              (`self.ExecuteHaptic` 0.01 _percent_4 Strength))))))))

(event `SetMeshVisibility`
  (params (Set :type Boolean))
  ;[1 1 1] Set Visibility
)

(event `ExecuteHaptic`
  (params (Frequency :type "Float (double-precision)" :default 0.01) (Amplitude :type "Float (double-precision)") (StengthMultiplyer :type "Float (double-precision)"))
  ;[1 1 1] Haptics
  (bind _asbp_player_controller_main (cast `/Game/AVRFramework/Blueprints/Game/BP_PlayerController_Main` (`Pawn.GetController` (`self.VRPawn`))))
  (`PlayerController.SetHapticsByValue` _asbp_player_controller_main Frequency (* Amplitude StengthMultiplyer (`/Game/AVRFramework/DataAsset/Presets/VRControls/PDA_ControllerVR.HapticsMultiplyer` (`/Game/AVRFramework/Blueprints/Components/Info/Comp_Controls.getPresetAsset` (`/Game/AVRFramework/Blueprints/Pawn/BP_Pawn_VR.Comp_Controller_VR` (`self.VRPawn`))))) (select `/Game/AVRFramework/Enums/Enum_Side` (`self.Side`) :`NewEnumerator0` "Left" :`NewEnumerator1` "Right" :!type "EControllerHand Enum")))

(fn `getAllAttachedActors`
  (returns (Actors :type "Set of Actor Object Reference"))
  (locals (Return :type "Set of Actor Object Reference"))
  (bind _return (`local.Return`))
  (bind _values (`BlueprintMapLibrary.Map_Values` (`self.MCompMap`)))
  (for _array_element _values
    (`/Engine/EditorBlueprintResources/StandardMacros.IsValid` _array_element
      (:`Is Valid`
        (bind _actors (`/Game/AVRFramework/Blueprints/VR/MotionComponents/BP_MComp.getAllAttachedActors` _array_element))
        (`BlueprintSetLibrary.Set_Union` _return _actors)
        (`BlueprintSetLibrary.Set_Add` _return _array_element))))
  (return (`local.Return`)))

(fn `GribAxis`
  (params (AxisValue :type "Float (double-precision)"))
  (set `self.Axis_Grib` AxisValue))

(fn `SetThumbstickRotation`
  (params (InRotation :type "Rotator Structure") (InRotationNoOffset :type "Rotator Structure") (InUpAxis :type "Float (double-precision)") (InRightAxis :type "Float (double-precision)"))
  (locals (LocalUpAxis :type "Float (double-precision)") (LocalRightAxis :type "Float (double-precision)") (LocalRotation :type "Rotator Structure") (LocalRotationNoOffset :type "Rotator Structure"))
  (set `local.LocalRotation` InRotation)
  (set `local.LocalRotationNoOffset` InRotationNoOffset)
  (set `local.LocalUpAxis` InUpAxis)
  (set `local.LocalRightAxis` InRightAxis)
  (set `self.ThumbstickRotation` (`local.LocalRotation`))
  (set `self.ThumbstickRotationNoOffset` (`local.LocalRotationNoOffset`))
  (set `self.Axis_Thumbstick_Up` (`local.LocalUpAxis`))
  (set `self.Aixs_Thumbstick_Right` (`local.LocalRightAxis`)))

(fn `ThumbCapTouch`
  (params (AxisValue :type "Float (double-precision)"))
  (set `self.Axis_Thumb_Touch` AxisValue))

(fn `TriggerAxis`
  (params (AxisValue :type "Float (double-precision)"))
  (set `self.Axis_Trigger` AxisValue))

(fn `TriggerCapTouch`
  (params (AxisValue :type "Float (double-precision)"))
  (set `self.Axis_Trigger_Touch` AxisValue))

(fn `UserConstructionScript`)