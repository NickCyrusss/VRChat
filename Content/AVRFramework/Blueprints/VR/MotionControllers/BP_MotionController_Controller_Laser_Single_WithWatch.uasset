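; Motion controller Blueprint for VR, a single-laser "WithWatch" variant that refines when its laser is active.
; It overrides ShouldLaserBeActive, keeping the parent check and adding a condition for the left side only.
; On the left, a grabbed actor whose Comp_Grab has SnapAndReplaceControls set turns the laser off; the right follows the parent result.
; BeginPlay, Tick and construction only call the parent.
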(event `self.ReceiveBeginPlay`
  (`parent.ReceiveBeginPlay`))

(event `self.ReceiveTick`
  (params (DeltaSeconds :type "Float (single-precision)"))
  (`parent.ReceiveTick` DeltaSeconds))

(fn `ShouldLaserBeActive`
  (returns (ShouldBeActive :type Boolean))
  (if (`parent.ShouldLaserBeActive`)
    (switch `/Game/AVRFramework/Enums/Enum_Side` (`self.Side`)
      (:`NewEnumerator0`
        (bind _grabbedactor (message `/Game/AVRFramework/Interface/Interface_GrabbingActor.GrabbingActor_getCurrentlyGrabbedActor` (`BlueprintMapLibrary.Map_Find` (`self.MCompMap`) "NewEnumerator2")))
        (`/Engine/EditorBlueprintResources/StandardMacros.IsValid` _grabbedactor
          (:`Is Valid`
            (return (not (`/Game/AVRFramework/Blueprints/Components/Interaction/Comp_Grab.SnapAndReplaceControls` (`self.GetComponentByClass` _grabbedactor "/Game/AVRFramework/Blueprints/Components/Interaction/Comp_Grab.Comp_Grab_C")))))
          (:`Is Not Valid`
            _)))
      (:`NewEnumerator1`
        _))
    (return true)
    (else
      (return false))))

(fn `UserConstructionScript`
  (`parent.UserConstructionScript`))