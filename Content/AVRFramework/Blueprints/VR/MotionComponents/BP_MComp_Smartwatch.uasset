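; VR smartwatch motion component that spawns and dismisses a floating BP_Display on Display input, remembering its last content tab.
; An ungrabbed display follows the watch's hover point, while thumbstick up raises it to an eye-height, camera-facing position and down returns it to mini.
; Display map events also switch positions, including a tilted one.
; Timeline transitions blend toward a live-updated target, and a second timeline carries residual momentum afterwards.
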(event `self.ReceiveBeginPlay`
  (bind _vrpawn (`self.VRPawn`))
  (`parent.ReceiveBeginPlay`)
  (`/Game/AVRFramework/Libraries/MLib_Actor_Macros.WaitForObjectToValidate` _vrpawn
    (:`Is Valid`
      (set `self.ContentWidget` (`/Game/AVRFramework/Blueprints/Components/Info/Comp_UI_Display.InitialTab` (`self.GetComponentByClass` _vrpawn "/Game/AVRFramework/Blueprints/Components/Info/Comp_UI_Display.Comp_UI_Display_C"))))))

(event `SetSmallWidget`
  (params (Set :type Boolean))
  (if Set
    _))

(event `SetNewDisplayPosition`
  (params (DisplayPosition :type "/Game/AVRFramework/Enums/Enum_Display_Positions Enum" :default "NewEnumerator0"))
  ;[1 1 1] Initiate Move
  (if (`|EnumInequality` DisplayPosition (`self.DisplayPosition`))
    (set `self.DisplayPosition` DisplayPosition)
    (`self.MoveDisplay`)))

(event `self.ReceiveTick`
  (params (DeltaSeconds :type "Float (single-precision)"))
  (bind _thumbstickupaxis (`self.ThumbstickUpAxis`))
  (bind _display (`self.Display`))
  (bind _display_2 (`self.Display`))
  (bind (_returnvalue_location _returnvalue_rotation) (`KismetMathLibrary.BreakTransform` (`SceneComponent.K2_GetComponentToWorld` (`self.DisplayHover`))))
  (bind (_returnvalue_location_2 _returnvalue_rotation_2 _returnvalue_scale) (`KismetMathLibrary.BreakTransform` (`SceneComponent.K2_GetComponentToWorld` (`self.DisplayPortraitHandle`))))
  (bind _returnvalue (`SceneComponent.K2_GetComponentLocation` (`/Game/AVRFramework/Blueprints/Pawn/BP_Pawn_Base.GetCameraComponent` (`self.VRPawn`))))
  (bind (_returnvalue_roll _returnvalue_pitch _returnvalue_yaw) (`KismetMathLibrary.BreakRotator` (`KismetMathLibrary.FindLookAtRotation` _returnvalue_location_2 _returnvalue)))
  ;[1 1 1] Display Behaviour
  (`parent.ReceiveTick` DeltaSeconds)
  (`|ExecutionSequence`
    (:`then_0`
      (`/Engine/EditorBlueprintResources/StandardMacros.IsValid` (`self.Display`)
        (:`Is Valid`
          (if (`|EnumEquality` (`self.DisplayPosition`) "NewEnumerator1")
            (if (not (`self.InTransition`))
              (bind _grabbingpawn (`/Game/AVRFramework/Blueprints/Components/Interaction/Comp_Grab.CurrentlyGrabbedBy` (`/Game/AVRFramework/Blueprints/UI/InfoWindows/BP_Display.Comp_Grab` _display_2)))
              (`/Engine/EditorBlueprintResources/StandardMacros.IsValid` _grabbingpawn
                (:`Is Not Valid`
                  (`self.K2_SetActorLocationAndRotation` (`self.Display`) (`KismetMathLibrary.VInterpTo` (`self.K2_GetActorLocation` _display_2) _returnvalue_location DeltaSeconds 10.0) (`KismetMathLibrary.RInterpTo` (`self.K2_GetActorRotation` (`self.Display`)) _returnvalue_rotation DeltaSeconds 10.0) false false))))))))
    (:`then_1`
      (`/Engine/EditorBlueprintResources/StandardMacros.IsValid` _display
        (:`Is Valid`
          (`/Engine/EditorBlueprintResources/StandardMacros.IsValid` (`/Game/AVRFramework/Blueprints/Components/Interaction/Comp_Grab.GrabbingPawn` (`self.GetComponentByClass` _display "/Game/AVRFramework/Blueprints/Components/Interaction/Comp_Grab.Comp_Grab_C"))
            (:`Is Not Valid`
              (if (> _thumbstickupaxis 0.2)
                (`self.SetNewDisplayPosition` "NewEnumerator2")
                (`self.K2_SetActorTransform` (`self.Display`) (`KismetMathLibrary.TInterpTo` (`self.GetTransform` (`self.Display`)) (`KismetMathLibrary.MakeTransform` (`KismetMathLibrary.MakeVector` (.x _returnvalue_location_2) (.y _returnvalue_location_2) (.z _returnvalue)) (`KismetMathLibrary.MakeRotator` 0.0 0.0 _returnvalue_yaw) _returnvalue_scale) DeltaSeconds 4.0) false false)
                (elif (< _thumbstickupaxis -0.2)
                  (`self.SetNewDisplayPosition` "NewEnumerator1"))))))))))

(event `MoveDisplay`
  (bind (_returnvalue_location _returnvalue_rotation _returnvalue_scale) (`KismetMathLibrary.BreakTransform` (`SceneComponent.K2_GetComponentToWorld` (`self.DisplayPortraitHandle`))))
  (bind _returnvalue (`SceneComponent.K2_GetComponentLocation` (`/Game/AVRFramework/Blueprints/Pawn/BP_Pawn_Base.GetCameraComponent` (`self.VRPawn`))))
  (bind (_returnvalue_roll _returnvalue_pitch _returnvalue_yaw) (`KismetMathLibrary.BreakRotator` (`KismetMathLibrary.FindLookAtRotation` _returnvalue_location _returnvalue)))
  (bind _returnvalue_2 (select `/Game/AVRFramework/Enums/Enum_Display_Positions` (`self.DisplayPosition`) :`NewEnumerator0` (`SceneComponent.K2_GetComponentToWorld` (`self.DisplayStart`)) :`NewEnumerator1` (`SceneComponent.K2_GetComponentToWorld` (`self.DisplayHover`)) :`NewEnumerator2` (`KismetMathLibrary.MakeTransform` (`KismetMathLibrary.MakeVector` (.x _returnvalue_location) (.y _returnvalue_location) (.z _returnvalue)) (`KismetMathLibrary.MakeRotator` 0.0 0.0 _returnvalue_yaw) _returnvalue_scale) :`NewEnumerator3` (`SceneComponent.K2_GetComponentToWorld` (`self.DisplayTiltedHandle`))))
  ;[1 1 1] Display Move Logic (Super Customary)
  (bind _out (`/Game/AVRFramework/Libraries/FLib_Utility.SaveTransform` (`self.GetTransform` (`self.Display`))))
  (set `self.InTransition` true)
  (set `self.FollowValue` _returnvalue_2)
  (`TimelineComponent.SetPlayRate` (`self.MoveTimeline`) (select `/Game/AVRFramework/Enums/Enum_Display_Positions` (`self.DisplayPosition`) :`NewEnumerator0` 2.0 :`NewEnumerator1` 1.5 :`NewEnumerator2` 1.0 :`NewEnumerator3` 1.0 :!type "Float (single-precision)"))
  (bind (_direction _percent) (`Timeline|MoveTimeline` :!via `PlayFromStart`)
    (:`Update`
      (`/Engine/EditorBlueprintResources/StandardMacros.IsValid` (`self.Display`)
        (:`Is Valid`
          (set `self.FollowValue` (`KismetMathLibrary.TInterpTo` (`self.FollowValue`) _returnvalue_2 (`GameplayStatics.GetWorldDeltaSeconds`) 5.0))
          (bind _out_2 (`/Game/AVRFramework/Libraries/FLib_Utility.SaveVector` (`self.K2_GetActorLocation` (`self.Display`))))
          (`self.K2_SetActorTransform` (`self.Display`) (`KismetMathLibrary.TLerp` _out (`self.FollowValue`) _percent) false false))))
    (:`Finished`
      (`/Engine/EditorBlueprintResources/StandardMacros.IsValid` (`self.Display`)
        (:`Is Valid`
          (set `self.InTransition` false)
          (`self.Break` (- (`self.K2_GetActorLocation` (`self.Display`)) _out_2)))))
    (:`LerpOver`
      (switch `/Game/AVRFramework/Enums/Enum_Display_Positions` (`self.DisplayPosition`)
        (:`NewEnumerator0`
          (`/Game/AVRFramework/Libraries/FLib_Utility.DeleteActor` (`self.Display`))
          (set `self.Display` null)
          (`self.SetSmallWidget` true))))))

(event `Break`
  (params (InitialMovement :type "Vector Structure"))
  ;[1 1 1] Display Move Logic (Super Customary)
  (bind (_direction _procent) (`Timeline|StopTimeline` :!via `PlayFromStart`)
    (:`Update`
      (`/Engine/EditorBlueprintResources/StandardMacros.IsValid` (`self.Display`)
        (:`Is Valid`
          (`self.K2_SetActorLocation` (`self.Display`) (+ (`self.K2_GetActorLocation` (`self.Display`)) (* (* InitialMovement _procent) (`GameplayStatics.GetWorldDeltaSeconds`))) false false))))))

(event `MapAction`
  (params (Event :type "/Game/AVRFramework/Enums/Enum_Display_Events Enum" :default "NewEnumerator0"))
  ;[1 1 1] Appear on Highlight
  (switch `/Game/AVRFramework/Enums/Enum_Display_Events` Event
    (:`NewEnumerator1`
      (`/Game/AVRFramework/Blueprints/UI/InfoWindows/BP_Display.Set3DMap` (`self.Display`) true)
      (if (`|EnumEquality` (`self.DisplayPosition`) "NewEnumerator2")
        (`self.SetNewDisplayPosition` "NewEnumerator3")))
    (:`NewEnumerator2`
      (`/Game/AVRFramework/Blueprints/UI/InfoWindows/BP_Display.Set3DMap` (`self.Display`) true)
      (`self.SetNewDisplayPosition` "NewEnumerator1"))))

(event `ContentWidgetSwitched`
  (params (DisplayContent :type "/Game/AVRFramework/Blueprints/Widgets/Display/Widget_Display_Content Class Reference"))
  ;[1 1 1] Appear on Highlight
  (set `self.ContentWidget` DisplayContent))

(event `self.FunctionInput`
  (params (Function :type "/Game/AVRFramework/Enums/Enum_Control_Function Enum" :default "NewEnumerator0") (Set :type Boolean))
  ;[1 1 1] Appear on Highlight
  (`parent.FunctionInput` Function Set)
  (switch `/Game/AVRFramework/Enums/Enum_Control_Function` Function
    (:`NewEnumerator8`
      (if Set
        (`/Engine/EditorBlueprintResources/StandardMacros.IsValid` (`self.Display`)
          (:`Is Valid`
            (remove `/Game/AVRFramework/Blueprints/UI/InfoWindows/BP_Display.WidgetContentSwitched` (`self.Display`) (delegate `ContentWidgetSwitched`))
            (remove `/Game/AVRFramework/Blueprints/UI/InfoWindows/BP_Display.MapAction` (`self.Display`) (delegate `MapAction`))
            (`self.SetNewDisplayPosition` "NewEnumerator0"))
          (:`Is Not Valid`
            (bind _returnvalue (`|SpawnActorFromClass` "/Game/AVRFramework/Blueprints/UI/InfoWindows/BP_Display.BP_Display_C" (`SceneComponent.K2_GetComponentToWorld` (`self.DisplayStart`)) "AlwaysSpawn" "OverrideRootScale" null (`self.VRPawn`) (`self.ContentWidget`) null))
            (bind _output_get (set `self.Display` _returnvalue))
            (add `/Game/AVRFramework/Blueprints/UI/InfoWindows/BP_Display.WidgetContentSwitched` _output_get (delegate `ContentWidgetSwitched`))
            (`self.SetNewDisplayPosition` "NewEnumerator1")
            (`self.SetSmallWidget` false)
            (add `/Game/AVRFramework/Blueprints/UI/InfoWindows/BP_Display.MapAction` (`self.Display`) (delegate `MapAction`))))))))

(fn `Setup`
  (params (Side :type "/Game/AVRFramework/Enums/Enum_Side Enum" :default "NewEnumerator0") (VRPawn :type "/Game/AVRFramework/Blueprints/Pawn/BP_Pawn_VR Object Reference") (MotionComponent :type "MotionControllerComponent Object Reference") (MotionContoller :type "/Game/AVRFramework/Blueprints/VR/MotionControllers/BP_MotionController Object Reference"))
  (returns (Success :type Boolean))
  (bind _success (`parent.Setup` Side VRPawn MotionComponent MotionContoller))
  (switch `/Game/AVRFramework/Enums/Enum_Side` (`self.Side`)
    (:`NewEnumerator0`
      _)
    (:`NewEnumerator1`
      (`SceneComponent.K2_SetRelativeRotation` (`self.SmartWatch`) (struct :`Yaw` 180.0) false false)))
  (return _success))

(fn `UserConstructionScript`
  (`parent.UserConstructionScript`))