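; BP_Helper_MeasurementConnection draws a red laser between two measurement markers and labels its length in centimeters or meters.
; It drives a child BP_Helper_Laser, smoothing the forward vector with VInterpTo and placing the text at the spline midpoint.
; Tick turns the label toward the pawn camera and updates the connection only while a marker moves or the length is still settling.
; A looping timer also refreshes it periodically as a safety check.
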(event `self.ReceiveBeginPlay`
  (bind _asbp_helper_laser (cast `/Game/AVRFramework/Blueprints/Helpers/BP_Helper_Laser` (`ChildActorComponent.ChildActor` (`self.ChildActor`))))
  (bind _output_get (set `self.Laser` _asbp_helper_laser))
  (`/Game/AVRFramework/Blueprints/Helpers/BP_Helper_Laser.SetLaserColor` _output_get 0.0 0.0 false (struct :`R` 1.0 :`A` 1.0) 1.0 (1.0 1.0) (1.0 1.0) true)
  (`KismetSystemLibrary.K2_SetTimerDelegate` (delegate `CheckIfLaserStillWorksRight`) 5.0 true))

(event `CheckIfLaserStillWorksRight`
  (bind _returnvalue (`SceneComponent.K2_GetComponentLocation` (`/Game/AVRFramework/Blueprints/Helpers/BP_Helper_MeasurementMarker.LaserLocation` (`self.MeasurementMarkerA`))))
  (bind _returnvalue_2 (`SceneComponent.K2_GetComponentLocation` (`/Game/AVRFramework/Blueprints/Helpers/BP_Helper_MeasurementMarker.LaserLocation` (`self.MeasurementMarkerB`))))
  (bind _returnvalue_3 (`SplineComponent.GetSplineLength` (`/Game/AVRFramework/Blueprints/Helpers/BP_Helper_Laser.HelperSpline` (`self.Laser`))))
  (bind _returnvalue_4 (`SplineComponent.GetSplineLength` (`/Game/AVRFramework/Blueprints/Helpers/BP_Helper_Laser.HelperSpline` (`self.Laser`))))
  (bind _returnvalue_5 (>= _returnvalue_4 100.0))
  (bind _returnvalue_6 (select `bool` _returnvalue_5 :`false` 1 :`true` 2))
  (bind _output_get (set `self.LastForwardVector` (`KismetMathLibrary.VInterpTo` (`self.LastForwardVector`) (`KismetMathLibrary.Normal` (- _returnvalue_2 _returnvalue)) (stale `self.ReceiveTick` DeltaSeconds) 2.0) :!label _label))
  (`/Game/AVRFramework/Blueprints/Helpers/BP_Helper_Laser.UpdateLaser` (`self.Laser`) _returnvalue _returnvalue_2 _output_get)
  (set `self.LengthStillChanging` (not (`KismetMathLibrary.NearlyEqual_FloatFloat` (`self.CurrentLength`) _returnvalue_3 0.001)))
  (set `self.CurrentLength` _returnvalue_3)
  (`SceneComponent.K2_SetWorldLocation` (`self.TextHandle`) (`SplineComponent.GetLocationAtDistanceAlongSpline` (`/Game/AVRFramework/Blueprints/Helpers/BP_Helper_Laser.HelperSpline` (`self.Laser`)) (/ (`self.CurrentLength`) 2.0) "Local") false false)
  (`TextRenderComponent.K2_SetText` (`self.DistanceText`) (`|FormatText` "{Length}{unit}" (`KismetTextLibrary.Conv_DoubleToText` (select `bool` _returnvalue_5 :`false` _returnvalue_4 :`true` (/ _returnvalue_4 100.0)) "HalfToEven" false true 1 324 _returnvalue_6 _returnvalue_6) (select `bool` _returnvalue_5 :`false` "cm" :`true` "m"))))

(event `self.ReceiveTick`
  (params (DeltaSeconds :type "Float (single-precision)"))
  (`SceneComponent.K2_SetWorldRotation` (`self.TextHandle`) (`KismetMathLibrary.FindLookAtRotation` (`SceneComponent.K2_GetComponentLocation` (`self.TextHandle`)) (`SceneComponent.K2_GetComponentLocation` (`/Game/AVRFramework/Blueprints/Pawn/BP_Pawn_Base.GetCameraComponent` (`self.Pawn`)))) false false)
  (bind _inmotion (`/Game/AVRFramework/Blueprints/Helpers/BP_Helper_MeasurementMarker.IsInMotion` (`self.MeasurementMarkerB`)))
  (if _inmotion
    (goto _label)
    (else
      (bind _inmotion_2 (`/Game/AVRFramework/Blueprints/Helpers/BP_Helper_MeasurementMarker.IsInMotion` (`self.MeasurementMarkerA`)))
      (if _inmotion_2
        (goto _label)
        (elif (`self.LengthStillChanging`)
          (goto _label))))))

(fn `UserConstructionScript`)