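; BP_Helper_TransferPawn is a temporary pawn that hands a player over to their spawned pawn.
; On BeginPlay, when locally controlled, it sets the camera to black and calls ServerSpawnPawn.
; That event gets a player index from BP_GameMode_Main and passes it, with the current level key, to the player controller's ClientSpawnPawn.
; The helper destroys itself once unpossessed.
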(event `self.ReceiveTick`
  (params (DeltaSeconds :type "Float (single-precision)")))

(event `ServerSpawnPawn`
  (params (Controller :type "Controller Object Reference"))
  (bind _asbp_game_mode_main (cast `/Game/AVRFramework/Blueprints/Game/BP_GameMode_Main` (`GameplayStatics.GetGameMode`)))
  (bind _asbp_player_controller_main (cast `/Game/AVRFramework/Blueprints/Game/BP_PlayerController_Main` Controller))
  (bind _newindex (`/Game/AVRFramework/Blueprints/Game/BP_GameMode_Main.CreatePlayerIndex` _asbp_game_mode_main _asbp_player_controller_main))
  (`/Game/AVRFramework/Blueprints/Game/BP_PlayerController_Main.Client_SpawnPawn` _asbp_player_controller_main _newindex (`/Game/AVRFramework/Libraries/Lib_Core.getCurrentLevel` self)))

(event `self.ReceiveBeginPlay`
  (bind _returnvalue (`self.GetController`))
  (if (`self.IsLocallyControlled`)
    (`|ExecutionSequence`
      (:`then_0`
        (bind _asbp_player_controller_main (cast `/Game/AVRFramework/Blueprints/Game/BP_PlayerController_Main` _returnvalue))
        (`PlayerCameraManager.SetManualCameraFade` :`self` (`PlayerController.PlayerCameraManager` _asbp_player_controller_main) :`InFadeAmount` 1.0))
      (:`then_1`
        (`self.ServerSpawnPawn` _returnvalue)))))

(event `self.ReceivePossessed`
  (params (NewController :type "Controller Object Reference")))

(event `self.ReceiveUnpossessed`
  (params (OldController :type "Controller Object Reference"))
  (`self.K2_DestroyActor`))

(fn `UserConstructionScript`)