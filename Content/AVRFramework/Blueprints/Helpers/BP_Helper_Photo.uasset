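; BP_Helper_Photo is an AVRFramework helper actor that represents a photo on a plane and can export it as a PNG.
; PrintPicture creates a render target, binds it to a dynamic material on the plane, records the timecode and returns the target.
; ExportPhoto saves that target under a timestamp-based filename in the level info's export path and returns the file path.
; GetPhoto exposes the plane's material.
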(event `self.ReceiveTick`
  (params (DeltaSeconds :type "Float (single-precision)")))

(event `self.ReceiveBeginPlay`)

(fn `ExportPhoto`
  (returns (Path :type String))
  (bind (_returnvalue_year _returnvalue_month _returnvalue_day _returnvalue_hour _returnvalue_minute _returnvalue_second) (`KismetMathLibrary.BreakDateTime` (`KismetMathLibrary.Now`)))
  (bind _returnvalue (`KismetStringLibrary.Concat_StrStr` "Screen_" (`KismetStringLibrary.Conv_IntToString` _returnvalue_day) (`KismetStringLibrary.Conv_IntToString` _returnvalue_hour) (`KismetStringLibrary.Conv_IntToString` _returnvalue_minute) (`KismetStringLibrary.Conv_IntToString` _returnvalue_second) ".png"))
  (bind _exportpath (`/Game/AVRFramework/Blueprints/Info/BP_Info_Level.ExportPath` (`/Game/AVRFramework/Libraries/Lib_Core.getInfoLevels` self)))
  ;[1 1 1] Export Picture to FilePath defined in the Universal Object
  (`KismetRenderingLibrary.ExportRenderTarget` (`self.TextureTarget`) _exportpath _returnvalue)
  (return (`KismetStringLibrary.Concat_StrStr` _exportpath "/" _returnvalue)))

(fn `getPhoto`
  (returns (ReturnValue :type "MaterialInterface Object Reference"))
  (return (`PrimitiveComponent.GetMaterial` (`self.Plane`) 0)))

(fn `PrintPicture`
  (returns (TextureTarget :type "TextureRenderTarget2D Object Reference"))
  (bind _returnvalue (`KismetRenderingLibrary.CreateRenderTarget2D` 800 500 "RTF_RGBA8"))
  (set `self.TextureTarget` _returnvalue)
  ;[1 1 1] Create Photo Instance with the Photo Material
  (bind _returnvalue_2 (`PrimitiveComponent.CreateDynamicMaterialInstance` (`self.Plane`) 0 null "None"))
  (`MaterialInstanceDynamic.SetTextureParameterValue` _returnvalue_2 "Texture" _returnvalue)
  (set `self.Time` (`TimeManagementBlueprintLibrary.GetTimecode`))
  (return _returnvalue))

(fn `UserConstructionScript`)