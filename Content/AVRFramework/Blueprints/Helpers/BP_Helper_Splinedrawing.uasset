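; Helper actor that draws a brush stroke as a spline built from pen positions passed to NewPenLocation.
; Each point added, at the start or once the pen exceeds scale-adjusted spacing from the second-last point, gets a new brush spline mesh with the given material.
; Otherwise the last point follows the pen.
; The newest mesh is refitted between the last two points, using spline directions as tangents and the given scale as width.
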(event `NewPenLocation`
  (params (Position :type "Vector Structure") (SplineMaterial :type "MaterialInterface Object Reference") (Scale :type "Float (double-precision)"))
  (bind _scale (`self.Scale`))
  (bind _spline (`self.Spline`))
  (bind _spline_2 (`self.Spline`))
  (bind _newestsplinemeshcomponent (`self.NewestSplineMeshComponent`))
  (bind _spline_3 (`self.Spline`))
  (bind _returnvalue (`SplineComponent.GetNumberOfSplinePoints` (`self.Spline`)))
  (bind _returnvalue_2 (- _returnvalue 2))
  (bind _returnvalue_3 (- _returnvalue 1))
  (set `self.SplineMaterial` SplineMaterial)
  (bind _output_get (set `self.CurrentSplineInt` (`SplineComponent.GetNumberOfSplinePoints` (`self.Spline`))))
  (if (<= _output_get 1)
    (`SplineComponent.AddSplinePoint` _spline_3 Position "World" true :!label _label)
    (`SplineComponent.SetSplinePointType` _spline_3 (- (`SplineComponent.GetNumberOfSplinePoints` (`self.Spline`)) 1) "Curve" true)
    (bind _returnvalue_4 (`AddComponent|NODE_AddSplineMeshComponent-1` :`bManualAttachment` true))
    (`SceneComponent.K2_AttachToComponent` _returnvalue_4 (`self.Scene`) "None" "KeepWorld" "KeepWorld" "KeepWorld" true)
    (set `self.NewestSplineMeshComponent` _returnvalue_4)
    (`StaticMeshComponent.SetStaticMesh` _newestsplinemeshcomponent "/Game/AVRFramework/Meshes/Devices/Drawing/Mesh_Tools_Drawing_Brush.Mesh_Tools_Drawing_Brush")
    (`PrimitiveComponent.SetMaterial` _newestsplinemeshcomponent 0 SplineMaterial)
    (elif (> (`/Game/AVRFramework/Libraries/FLib_Utility.DistanceBetweenVectors` Position (`SplineComponent.GetLocationAtSplinePoint` (`self.Spline`) (- (`self.CurrentSplineInt`) 2) "World")) (* (`self.spacing`) (`self.Scale`)))
      (goto _label)
      (else
        (`SplineComponent.SetLocationAtSplinePoint` (`self.Spline`) (- (`SplineComponent.GetNumberOfSplinePoints` (`self.Spline`)) 1) Position "World" true))))
  (`SplineMeshComponent.SetStartAndEnd` _newestsplinemeshcomponent (`SplineComponent.GetLocationAtSplinePoint` _spline _returnvalue_2 "World") (`SplineComponent.GetDirectionAtSplinePoint` _spline _returnvalue_2 "World") (`SplineComponent.GetLocationAtSplinePoint` _spline_2 _returnvalue_3 "World") (`SplineComponent.GetDirectionAtSplinePoint` _spline_2 _returnvalue_3 "World") true)
  (`SplineMeshComponent.SetStartScale` _newestsplinemeshcomponent (`KismetMathLibrary.MakeVector2D` _scale _scale) true)
  (bind _output_get_2 (set `self.Scale` Scale))
  (`SplineMeshComponent.SetEndScale` _newestsplinemeshcomponent (`KismetMathLibrary.MakeVector2D` _output_get_2 _output_get_2) true))

(fn `UserConstructionScript`)