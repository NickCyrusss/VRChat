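; VR helper actor that lets a grabbable object be pulled out of a holder component, shown shrunk until it is drawn away.
; While grabbed, Tick scales the object from a fitted size to full with distance, based on its largest static mesh's bounds.
; At full scale it restores collision, notifies Comp_Grab and destroys itself.
; Releasing earlier flies the object back on a distance-paced timeline, then deletes both actors.
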(event `self.ReceiveTick`
  (params (DeltaSeconds :type "Float (single-precision)"))
  ;[1 1 1] On Every Frame Adjust Size and check for detach
  (if (`self.Start`)
    (`/Engine/EditorBlueprintResources/StandardMacros.IsValid` (`self.AttachedActor`)
      (:`Is Valid`
        (bind _shoulddetach (`self.SetSizeToDistance`))
        (if _shoulddetach
          (`self.SetActorScale3D` (`self.AttachedActor`) (`KismetMathLibrary.Conv_DoubleToVector` 1.0))
          (`self.SetActorEnableCollision` (`self.AttachedActor`) true)
          (`/Game/AVRFramework/Blueprints/Components/Interaction/Comp_Grab.PullOver` (`self.GetComponentByClass` (`self.AttachedActor`) "/Game/AVRFramework/Blueprints/Components/Interaction/Comp_Grab.Comp_Grab_C"))
          (`self.K2_DestroyActor`))))))

(event `Released`
  (bind _attachedactor (`self.AttachedActor`))
  ;[1 1 1] Fly Back to Original Location
  (set `/Game/AVRFramework/Blueprints/Components/Interaction/Comp_Grab.CanbePickedUp` false (`self.GetComponentByClass` (`self.AttachedActor`) "/Game/AVRFramework/Blueprints/Components/Interaction/Comp_Grab.Comp_Grab_C"))
  (`PrimitiveComponent.SetSimulatePhysics` (cast `PrimitiveComponent` (`Actor.RootComponent` (`self.AttachedActor`)) :!pure true) false)
  (`TimelineComponent.SetPlayRate` (`self.FlyBackToPositionTimeline`) (`KismetMathLibrary.MapRangeClamped` (`/Game/AVRFramework/Libraries/FLib_Utility.DistanceBeweenTwoVectors` (`self.K2_GetActorLocation` (`self.AttachedActor`)) (`SceneComponent.K2_GetComponentLocation` (`self.MeshHandle`))) 10.0 1000.0 2.0 0.1))
  (bind _out (`/Game/AVRFramework/Libraries/FLib_Utility.SaveVector` (`self.K2_GetActorLocation` _attachedactor)))
  (bind _out_2 (`/Game/AVRFramework/Libraries/FLib_Utility.SaveRotator` (`self.K2_GetActorRotation` _attachedactor)))
  (bind (_direction _procent) (`Timeline|FlyBackToPositionTimeline` :!via `PlayFromStart` :!label _label)
    (:`Update`
      (`self.K2_SetActorLocationAndRotation` (`self.AttachedActor`) (`KismetMathLibrary.VLerp` _out (`self.K2_GetActorLocation`) _procent) (`KismetMathLibrary.RLerp` _out_2 (`self.K2_GetActorRotation`) _procent true) false false))
    (:`Finished`
      (`/Game/AVRFramework/Libraries/FLib_Utility.DeleteActor` (`self.AttachedActor`))
      (`/Game/AVRFramework/Libraries/FLib_Utility.DeleteActor` self))))

(event `Grabbed`
  (params (GrabbingPawn :type "/Game/AVRFramework/Blueprints/Pawn/BP_Pawn_Base Object Reference") (GrabbingActor :type "Actor Object Reference") (GrabbingMotionController :type "/Game/AVRFramework/Blueprints/VR/MotionControllers/BP_MotionController Object Reference") (GrabbingMComp :type "/Game/AVRFramework/Blueprints/VR/MotionComponents/BP_MComp Object Reference"))
  ;[1 1 1] Fly Back to Original Location
  (set `self.Start` true)
  (goto _label :!via `Stop`))

(event `self.ReceiveBeginPlay`
  (bind _returnvalue (`self.GetComponentByClass` (`self.AttachedActor`) "/Game/AVRFramework/Blueprints/Components/Interaction/Comp_Grab.Comp_Grab_C"))
  (`self.K2_AttachToComponent` (`self.ComponentToAttachTo`) "None" "KeepWorld" "KeepWorld" "KeepWorld")
  (`self.SetActorEnableCollision` (`self.AttachedActor`) false)
  (bind _component (`self.FindLargestComponent`))
  (set `self.MainComponent` _component)
  (`self.SetSizeToDistance`)
  (`/Engine/EditorBlueprintResources/StandardMacros.IsValid` _returnvalue
    (:`Is Valid`
      (set `/Game/AVRFramework/Blueprints/Components/Interaction/Comp_Grab.IsBeingPulled` true _returnvalue)
      (add `/Game/AVRFramework/Blueprints/Components/Interaction/Comp_Grab.ActorPickedUp` _returnvalue (delegate `Grabbed`))
      (add `/Game/AVRFramework/Blueprints/Components/Interaction/Comp_Grab.ActorReleased` _returnvalue (delegate `Released`)))))

(fn `FindLargestComponent`
  (returns (Component :type "StaticMeshComponent Object Reference"))
  (locals (Return :type "StaticMeshComponent Object Reference"))
  (for _array_element (`self.K2_GetComponentsByClass` (`self.AttachedActor`) "/Script/Engine.StaticMeshComponent")
    (`/Engine/EditorBlueprintResources/StandardMacros.IsValid` _array_element
      (:`Is Valid`
        (if (> (`KismetMathLibrary.VSize` (`.BoxExtent` (`KismetSystemLibrary.GetComponentBounds` _array_element))) (`KismetMathLibrary.VSize` (`.BoxExtent` (`KismetSystemLibrary.GetComponentBounds` (`local.Return`)))))
          (set `local.Return` _array_element)))))
  (return (`local.Return`)))

(fn `SetSizeToDistance`
  (returns (ShouldDetach :type Boolean))
  (bind (_min _max) (`StaticMeshComponent.GetLocalBounds` (`self.MainComponent`)))
  (bind _returnvalue (`KismetMathLibrary.FMax` (+ (`KismetMathLibrary.Abs` (.x _min)) (`KismetMathLibrary.Abs` (.x _max))) (+ (`KismetMathLibrary.Abs` (.y _min)) (`KismetMathLibrary.Abs` (.y _max))) (+ (`KismetMathLibrary.Abs` (.z _min)) (`KismetMathLibrary.Abs` (.z _max)))))
  (bind _returnvalue_2 (`KismetMathLibrary.MapRangeClamped` (`KismetMathLibrary.VSize` (- (`self.K2_GetActorLocation` (`self.AttachedActor`)) (`self.K2_GetActorLocation`))) 0.0 (`KismetMathLibrary.FClamp` (/ _returnvalue 1.5) 20.0 100.0) 0.0 1.0))
  (`self.SetActorScale3D` (`self.AttachedActor`) (`KismetMathLibrary.Conv_DoubleToVector` (`KismetMathLibrary.Lerp` (/ (`self.Size`) _returnvalue) 1.0 _returnvalue_2)))
  (return (>= _returnvalue_2 1.0)))

(fn `UserConstructionScript`)